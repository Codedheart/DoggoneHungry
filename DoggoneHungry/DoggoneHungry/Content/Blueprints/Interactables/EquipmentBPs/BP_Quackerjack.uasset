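; BP_Quackerjack is an interactable equipment item with a widget that displays its item information.
; On BeginPlay it casts the widget's user object to ObjectInformationDisplay and fills in the name and attribute enum from ItemInfo.
; ShowWidget and HideWidget events toggle the widget's visibility, and the construction script only calls its parent.
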(event Custom|ShowWidget
  (Rendering|SetVisibility (Variables|Default|GetWidget) true false))

(event Custom|HideWidget
  (Rendering|SetVisibility (Variables|Default|GetWidget) false false))

(event EventBeginPlay
  (bind _iteminfo (Variables|Default|GetItemInfo))
  (bind _asobject_information_display (Utilities|Casting|CastToObjectInformationDisplay (UserInterface|GetUserWidgetObject (Variables|Default|GetWidget))))
  (Variables|/Game/UI/Widgets/ObjectInformationDisplay.ObjectInformationDisplay_C|SetDisplayText _asobject_information_display (.name _iteminfo))
  (Variables|/Game/UI/Widgets/ObjectInformationDisplay.ObjectInformationDisplay_C|SetAttributeEnum _asobject_information_display (.attributeenum _iteminfo)))

(fn ConstructionScript
  (|CallParentFunction))