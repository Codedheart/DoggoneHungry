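; Interactable door Blueprint that any actor except BP_Dog toggles open and closed through UseInteract.
; A FlipFlop plays or reverses the OpenDoor timeline, which sets the mesh's relative yaw from the track value plus the actor yaw saved at construction.
; The open sound plays as opening starts, and the close sound when closing finishes.
; Construction also applies the door material; cached arrow locations and OpenRotation go unused in these graphs.
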(event EventBeginPlay
  (Variables|Default|SetInArrowLocation (Transformation|GetWorldLocation (Variables|Default|GetInArrow)))
  (Variables|Default|SetOutArrowLocation (Transformation|GetWorldLocation (Variables|Default|GetOutArrow))))

(event EventUseInteract
  (params (UsingActor :type Actor%20Object%20Reference))
  (bind _returnvalue (Transformation|GetActorLocation))
  (Utilities|Casting|CastToBP_Dog UsingActor
    (:CastFailed
      (bind _isa (Utilities|FlowControl|FlipFlop)
        (:A
          (Audio|PlaySoundatLocation "/Game/Sound/Items/Door/Door_Open_Cue.Door_Open_Cue" _returnvalue "0, 0, 0" 1.0 1.0 0.0 0 0 0)
          (bind _newtrack_0 (Timeline|OpenDoor Play)
            (:Update
              (Transformation|SetRelativeRotation (Variables|Default|GetStaticMesh) (Math|Rotator|MakeRotator 0.0 0.0 (+ _newtrack_0 (.Yaw (Math|Rotator|BreakRotator (Variables|Default|GetNewVar_0))))) false false))
            (:Finished
              (if (not _isa)
                (Audio|PlaySoundatLocation "/Game/Sound/Items/Door/Door_Close_Cue.Door_Close_Cue" _returnvalue "0, 0, 0" 1.0 1.0 0.0 0 0 0)))))
        (:B
          (Timeline|OpenDoor Reverse))))))

(fn ConstructionScript
  (bind _returnvalue (Transformation|GetActorRotation))
  (bind (_roll _pitch _yaw) (Math|Rotator|BreakRotator _returnvalue))
  (Rendering|Material|SetMaterial (Variables|Default|GetStaticMesh) 0 (Variables|Default|GetDoor%20Material))
  (Variables|Default|SetOpenRotation (Math|Rotator|MakeRotator _roll _pitch (+ _yaw 9e+01)))
  (Variables|Default|SetNewVar_0 _returnvalue))