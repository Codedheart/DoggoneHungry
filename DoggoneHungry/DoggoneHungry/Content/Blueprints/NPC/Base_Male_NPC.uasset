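; Base male NPC Blueprint that builds its look from modular bottom, top and hair skeletal meshes.
; The construction script assigns each part's mesh from a variable, so different meshes can be set per variant.
; All three parts use the main Mesh as master pose component, so they follow its animation.
; BeginPlay contains no logic.
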(event EventBeginPlay)

(fn ConstructionScript
  (Class|SkinnedMeshComponent|SetSkeletalMesh (Variables|Default|GetBOTTOM) (Variables|Default|GetBottomVar) true)
  (Class|SkinnedMeshComponent|SetSkeletalMesh (Variables|Default|GetTOP) (Variables|Default|GetTopVar) true)
  (Class|SkinnedMeshComponent|SetSkeletalMesh (Variables|Default|GetHAIR) (Variables|Default|GetHairVar) true)
  (Class|SkinnedMeshComponent|SetMasterPoseComponent (Variables|Default|GetTOP) (Variables|Character|GetMesh) false))