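; BP_T3_BalancedFood is a food actor that acts as a balanced item until it is told that balancing has failed.
; Every tick it resets its world rotation to zero using a physics teleport.
; The FailBalance event detaches it, keeping its world transform, then enables physics-only collision and simulation on BalancedMesh and applies a forward force.
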(event Custom|FailBalance
  (bind _balancedmesh (Variables|Default|GetBalancedMesh))
  (Transformation|DetachFromActor "KeepWorld" "KeepWorld" "KeepWorld")
  (Collision|SetCollisionEnabled _balancedmesh "PhysicsOnly")
  (Physics|SetSimulatePhysics _balancedmesh true)
  (Physics|AddForce _balancedmesh (* (Math|Vector|GetForwardVector _balancedmesh) 5e+02) "None" false))

(event EventBeginPlay)

(event Collision|EventActorBeginOverlap
  (params (OtherActor :type Actor%20Object%20Reference)))

(event EventTick
  (params (DeltaSeconds :type Float%20%28single-precision%29))
  (Transformation|SetActorRotation (Math|Rotator|MakeRotator 0.0 0.0 0.0) true))

(fn ConstructionScript)