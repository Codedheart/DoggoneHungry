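; BP_FridgeDoor is an interactable fridge door that slides open and closed and serves a dog ice cream objective.
; Interactors other than BP_Dog toggle it through a FlipFlop, playing or reversing a timeline that moves the mesh along world Y between its start position and OpenLocation.
; When BP_Dog interacts while the door is flagged open, a second mesh is destroyed and the dog's CanHandInIcecreamObjective flag is set.
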(event EventBeginPlay
  (Variables|Default|SetStartLocation (Transformation|GetWorldLocation (Variables|Default|GetStaticMesh))))

(event EventUseInteract
  (params (UsingActor :type Actor%20Object%20Reference))
  (bind _startlocation (Variables|Default|GetStartLocation))
  (bind _asbp_dog (Utilities|Casting|CastToBP_Dog UsingActor)
    (:then
      (if (Variables|Default|GetOpen/Closed)
        (Components|DestroyComponent (Variables|Default|GetStaticMesh1))
        (Variables|/Game/Player+AI/Blueprints/BP_Dog.BP_Dog_C|SetCanHandInIcecreamObjective _asbp_dog true)))
    (:CastFailed
      (Utilities|FlowControl|FlipFlop
        (:A
          (Variables|Default|SetOpen/Closed true)
          (bind _newtrack_0 (Timeline|Open Play)
            (:Update
              (Transformation|SetWorldLocation (Variables|Default|GetStaticMesh) (Math|Vector|MakeVector (.x _startlocation) (+ (* _newtrack_0 (- (.y (Variables|Default|GetOpenLocation)) (.y _startlocation))) (.y _startlocation)) (.z _startlocation)) false false))))
        (:B
          (Variables|Default|SetOpen/Closed false)
          (Timeline|Open Reverse))))))

(fn ConstructionScript)