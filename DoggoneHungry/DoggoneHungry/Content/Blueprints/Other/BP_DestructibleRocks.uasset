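; Rock obstacle made of four destructible components that break when BP_Dog hits them while its morph target value is almost at full (0.99 or above).
; A qualifying hit applies damage to that component to trigger fracturing.
; On fracture, the component ignores Pawn and Camera collision, and a timeline restarts to drive the Opacity material parameter on all four components, not only the broken one.
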(event OnComponentFracture(Destructible)
  (params (HitPoint :type Vector%20%28by%20ref%29 :default "0, 0, 0") (HitDirection :type Vector%20%28by%20ref%29 :default "0, 0, 0"))
  (CallFunction|IgnorePawn (Variables|Default|GetDestructible)))

(event OnComponentHit(Destructible)
  (params (HitComponent :type Primitive%20Component%20Object%20Reference) (OtherActor :type Actor%20Object%20Reference) (OtherComp :type Primitive%20Component%20Object%20Reference) (NormalImpulse :type Vector :default "0, 0, 0") (Hit :type Hit%20Result%20Structure%20%28by%20ref%29))
  (bind _asbp_dog (Utilities|Casting|CastToBP_Dog OtherActor))
  (if (>= (Variables|/Game/Player+AI/Blueprints/BP_Dog.BP_Dog_C|GetCurrentMorphTargetValue _asbp_dog) 0.99)
    (CallFunction|ApplyDestructible (Variables|Default|GetDestructible))))

(event OnComponentHit(Destructible1)
  (params (HitComponent :type Primitive%20Component%20Object%20Reference) (OtherActor :type Actor%20Object%20Reference) (OtherComp :type Primitive%20Component%20Object%20Reference) (NormalImpulse :type Vector :default "0, 0, 0") (Hit :type Hit%20Result%20Structure%20%28by%20ref%29))
  (bind _asbp_dog (Utilities|Casting|CastToBP_Dog OtherActor))
  (if (>= (Variables|/Game/Player+AI/Blueprints/BP_Dog.BP_Dog_C|GetCurrentMorphTargetValue _asbp_dog) 0.99)
    (CallFunction|ApplyDestructible (Variables|Default|GetDestructible1))))

(event OnComponentHit(Destructible2)
  (params (HitComponent :type Primitive%20Component%20Object%20Reference) (OtherActor :type Actor%20Object%20Reference) (OtherComp :type Primitive%20Component%20Object%20Reference) (NormalImpulse :type Vector :default "0, 0, 0") (Hit :type Hit%20Result%20Structure%20%28by%20ref%29))
  (bind _asbp_dog (Utilities|Casting|CastToBP_Dog OtherActor))
  (if (>= (Variables|/Game/Player+AI/Blueprints/BP_Dog.BP_Dog_C|GetCurrentMorphTargetValue _asbp_dog) 0.99)
    (CallFunction|ApplyDestructible (Variables|Default|GetDestructible2))))

(event OnComponentHit(Destructible3)
  (params (HitComponent :type Primitive%20Component%20Object%20Reference) (OtherActor :type Actor%20Object%20Reference) (OtherComp :type Primitive%20Component%20Object%20Reference) (NormalImpulse :type Vector :default "0, 0, 0") (Hit :type Hit%20Result%20Structure%20%28by%20ref%29))
  (bind _asbp_dog (Utilities|Casting|CastToBP_Dog OtherActor))
  (if (>= (Variables|/Game/Player+AI/Blueprints/BP_Dog.BP_Dog_C|GetCurrentMorphTargetValue _asbp_dog) 0.99)
    (CallFunction|ApplyDestructible (Variables|Default|GetDestructible3))))

(event OnComponentFracture(Destructible1)
  (params (HitPoint :type Vector%20%28by%20ref%29 :default "0, 0, 0") (HitDirection :type Vector%20%28by%20ref%29 :default "0, 0, 0"))
  (CallFunction|IgnorePawn (Variables|Default|GetDestructible1)))

(event OnComponentFracture(Destructible2)
  (params (HitPoint :type Vector%20%28by%20ref%29 :default "0, 0, 0") (HitDirection :type Vector%20%28by%20ref%29 :default "0, 0, 0"))
  (CallFunction|IgnorePawn (Variables|Default|GetDestructible2)))

(event OnComponentFracture(Destructible3)
  (params (HitPoint :type Vector%20%28by%20ref%29 :default "0, 0, 0") (HitDirection :type Vector%20%28by%20ref%29 :default "0, 0, 0"))
  (CallFunction|IgnorePawn (Variables|Default|GetDestructible3)))

(event Custom|ApplyDestructible
  (params (NewDestructible :type Destructible%20Component%20Object%20Reference))
  (bind _returnvalue (Transformation|GetWorldLocation NewDestructible))
  (Class|DestructibleComponent|ApplyDamage NewDestructible 1.0 _returnvalue _returnvalue 1.0))

(event Custom|IgnorePawn
  (params (NewDestructible :type Destructible%20Component%20Object%20Reference))
  (Collision|SetCollisionResponsetoChannel NewDestructible "ECC_Pawn" "ECR_Ignore")
  (Collision|SetCollisionResponsetoChannel NewDestructible "ECC_Camera" "ECR_Ignore")
  (CallFunction|UpdateOpacity))

(event Custom|UpdateOpacity
  (bind _opacity (Timeline|Timeline_0 PlayFromStart)
    (:Update
      (Rendering|Material|SetScalarParameterValueonMaterials (Variables|Default|GetDestructible) "Opacity" _opacity))))

(event EventBeginPlay)

(event Collision|EventActorBeginOverlap
  (params (OtherActor :type Actor%20Object%20Reference)))

(event EventTick
  (params (DeltaSeconds :type Float%20%28single-precision%29)))

(fn ConstructionScript)