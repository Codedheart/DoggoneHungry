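; BP_RaceFlag is a race checkpoint in a linked chain of flags that the dog passes through.
; It hides its two flags and plane on BeginPlay, and Activate shows them with the trigger box and enables its overlap events.
; When a BP_Dog allowed to race overlaps the box, the flag activates NextFlag, or marks the race objective ready to hand in if none exists, then destroys itself.
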(event OnComponentBeginOverlap(Box)
  (params (OverlappedComponent :type Primitive%20Component%20Object%20Reference) (OtherActor :type Actor%20Object%20Reference) (OtherComp :type Primitive%20Component%20Object%20Reference) (OtherBodyIndex :type Integer) (bFromSweep :type Boolean) (SweepResult :type Hit%20Result%20Structure%20%28by%20ref%29))
  (bind _asbp_dog (Utilities|Casting|CastToBP_Dog OtherActor))
  (if (Variables|/Game/Player+AI/Blueprints/BP_Dog.BP_Dog_C|GetbCanStartRace _asbp_dog)
    (if (Utilities|IsValid (Variables|Default|GetNextFlag))
      (CallFunction|Activate (Variables|Default|GetNextFlag))
      (else
        (Variables|/Game/Player+AI/Blueprints/BP_Dog.BP_Dog_C|SetbCanHandInRaceObjective _asbp_dog true)))
    (Actor|DestroyActor)))

(event Custom|Activate
  (Rendering|SetVisibility (Variables|Default|GetFlag2) true false)
  (Variables|/Script/Engine.PrimitiveComponent|SetbGenerateOverlapEvents (Variables|Default|GetBox) true))

(event EventBeginPlay
  (Rendering|SetVisibility (Variables|Default|GetFlag2) false false))

(event Collision|EventActorBeginOverlap
  (params (OtherActor :type Actor%20Object%20Reference)))

(event EventTick
  (params (DeltaSeconds :type Float%20%28single-precision%29)))

(fn ConstructionScript)