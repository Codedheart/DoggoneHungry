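; Behavior tree task that lets a guest AI find another guest to start a conversation with.
; It checks the busy flag of a random GuestArray entry and fails immediately if that guest is busy.
; Otherwise it marks itself and a partner busy, stores the partner on the blackboard, calls StartConversation and flags the conversation as started.
; The partner is drawn by a second random pick, so it can differ from the guest checked.
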(event EventReceiveExecuteAI
  (params (OwnerController :type AI%20Controller%20Object%20Reference) (ControlledPawn :type Pawn%20Object%20Reference))
  (bind _asguest_ai (Utilities|Casting|CastToGuestAI ControlledPawn))
  (if (ScalableFloat|GetValueasBool (AI|GetBlackboard (Utilities|Array|Get(acopy) (Variables|/Game/Player+AI/Blueprints/GuestAI.GuestAI_C|GetGuestArray _asguest_ai) (Math|Random|RandomInteger (Utilities|Array|Length (Variables|/Game/Player+AI/Blueprints/GuestAI.GuestAI_C|GetGuestArray _asguest_ai))))) (Variables|Default|GetisBusyKey))
    (AI|BehaviorTree|FinishExecute false)
    (else
      (bind _output_get (Variables|Default|SetPartner (Utilities|Array|Get(acopy) (Variables|/Game/Player+AI/Blueprints/GuestAI.GuestAI_C|GetGuestArray _asguest_ai) (Math|Random|RandomInteger (Utilities|Array|Length (Variables|/Game/Player+AI/Blueprints/GuestAI.GuestAI_C|GetGuestArray _asguest_ai))))))
      (Class|BTFunctionLibrary|SetBlackboardValueasObject (Variables|Default|GetConvoPartner) _output_get)
      (Class|BTFunctionLibrary|SetBlackboardValueasBool (Variables|Default|GetisBusy?) true)
      (AI|Components|Blackboard|SetValueasBool (AI|GetBlackboard _output_get) (Variables|Default|GetisBusyKey) true)
      (Default|StartConversation _output_get _asguest_ai)
      (Class|BTFunctionLibrary|SetBlackboardValueasBool (Variables|Default|GetStartedConvo) true)
      (AI|BehaviorTree|FinishExecute true))))