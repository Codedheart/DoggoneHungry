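; Behavior tree task that turns an AI pawn toward the player's location, read from a Blackboard vector key.
; It first saves the pawn's current rotation to the Blackboard so it can be resumed later.
; It then applies a single fixed-step RInterpTo toward the yaw-only look-at rotation and finishes immediately, so each execution turns only part of the way.
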(event EventReceiveExecuteAI
  (params (OwnerController :type AI%20Controller%20Object%20Reference) (ControlledPawn :type Pawn%20Object%20Reference))
  (bind _returnvalue (AI|GetBlackboard ControlledPawn))
  (bind _returnvalue_2 (Transformation|GetActorRotation ControlledPawn))
  ;[1 1 1] Gets look at rotation between AI and player and sets the AIs world rotation
  (Class|BlackboardComponent|SetValueasRotator _returnvalue (Variables|Default|GetInitialRotation_Key) _returnvalue_2) ; sets rotator for resumerotation
  (Transformation|SetActorRotation ControlledPawn (Math|Interpolation|RInterpTo _returnvalue_2 (Math|Rotator|MakeRotator 0.0 0.0 (.Yaw (Math|Rotator|BreakRotator (Math|Rotator|FindLookatRotation (Transformation|GetActorLocation ControlledPawn) (AI|Components|Blackboard|GetValueasVector _returnvalue (Variables|Default|GetLocation_Key)))))) 1.0 0.2))
  (AI|BehaviorTree|FinishExecute true))