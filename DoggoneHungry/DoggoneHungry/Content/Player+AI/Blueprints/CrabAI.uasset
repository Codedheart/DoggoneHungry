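; Crab enemy that patrols between PointA and PointB and catches the player dog when it notices it.
; A FlipFlop alternates AIMoveTo targets, while a timeline drives WalkFloat for animation.
; A looping timer runs a capsule trace, flagging the player if moving above sneak speed within an angle of the crab's right vector.
; A catch turns the dog's camera, calls Caught and briefly shows particles and a message, gated by DoOnce.
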(event Custom|CaughtDog!
  (bind _asbp_dog (Utilities|Casting|CastToBP_Dog (Game|GetPlayerCharacter 0)))
  (Utilities|FlowControl|DoOnce false :!label _label
    (:Completed
      (Default|RotateCameraTowardsEnemy _asbp_dog self)
      (Components|Activation|SetActive (Variables|Default|GetParticleSystem) true true)
      (Default|Caught _asbp_dog 2.5)
      (bind _returnvalue (UserInterface|CreateWidget "/Game/UI/Widgets/CaughtMessage.CaughtMessage_C" (Game|GetPlayerController 0)))
      (bind _output_get (Variables|Default|SetCaughtMessage _returnvalue))
      (UserInterface|Viewport|AddtoViewport _output_get 0)
      (Utilities|FlowControl|Delay 3.0)
      (Widget|RemovefromParent (Variables|Default|GetCaughtMessage))
      (Components|Activation|SetActive (Variables|Default|GetParticleSystem) false false)
      (goto _label Reset))))

(event Custom|PathBetweenTwoPoints
  (bind _self self)
  (Utilities|FlowControl|FlipFlop
    (:A
      (AI|AIMoveTo _self "0, 0, 0" (Variables|Default|GetPointA) 5.0 true
        (:OnSuccess
          (Utilities|FlowControl|Delay 1.0 :!label _label)
          (CallFunction|PathBetweenTwoPoints))
        (:OnFail
          (Development|PrintString "Pathing Failure" :!label _label_2))))
    (:B
      (AI|AIMoveTo _self "0, 0, 0" (Variables|Default|GetPointB) 5.0 true
        (:OnSuccess
          (goto _label))
        (:OnFail
          (goto _label_2))))))

(event Custom|StartAnimController
  (bind _walkanim (Timeline|CrabAnimController Play)
    (:Update
      (Variables|Default|SetWalkFloat _walkanim))))

(event EventBeginPlay
  (Utilities|Time|SetTimerbyFunctionName 0 "DetectionTrace" 0.1 true)
  (Actor|GetAllActorsOfClass "/Game/Blueprints/Other/CatSpawnPoint.CatSpawnPoint_C")
  (if (and (Utilities|IsValid (Variables|Default|GetPointA)) (Utilities|IsValid (Variables|Default|GetPointB)))
    (CallFunction|PathBetweenTwoPoints)
    (CallFunction|StartAnimController)
    (else
      (Development|PrintString "Warning: Crab path not set."))))

(fn ConstructionScript)

(fn DetectionTrace
  (bind _returnvalue (Transformation|GetActorRightVector))
  (bind _returnvalue_2 (Transformation|GetActorLocation))
  (bind _returnvalue_3 (Transformation|GetActorLocation))
  (bind _returnvalue_4 (Game|Player|GetPlayerPawn 0))
  (bind _returnvalue_5 (Game|Player|GetPlayerPawn 0))
  (bind _returnvalue_6 (Transformation|GetActorLocation _returnvalue_5))
  (bind _returnvalue_7 (Math|Vector|GetUnitDirection(Vector) _returnvalue_3 _returnvalue_6))
  (bind _outhits (Class|KismetSystemLibrary|CapsuleTraceMultiforObjects _returnvalue_2 _returnvalue_2 2.8e+02 1e+03 (Utilities|Array|MakeArray "ObjectTypeQuery3") false (Utilities|Array|MakeArray self) "None" true))
  (for _array_element _outhits
    (if (== (.HitActor (Collision|BreakHitResult _array_element)) _returnvalue_5)
      (if (and (> (Math|Vector|VectorLength (Transformation|GetVelocity _returnvalue_4)) (+ (Variables|/Game/Player+AI/Blueprints/BP_Dog.BP_Dog_C|GetSneakSpeed (.AsBP%20Dog (Utilities|Casting|CastToBP_Dog _returnvalue_4))) 1.0)) (< (Class|KismetMathLibrary|DegAcos (Math|Vector|DotProduct (Math|Vector|MakeVector (.x _returnvalue_7) (.y _returnvalue_7) 0.0) (Math|Vector|MakeVector (.x _returnvalue) (.y _returnvalue) 0.0))) (Variables|Default|GetDetectionDegree)))
        (CallFunction|CaughtDog!)))))