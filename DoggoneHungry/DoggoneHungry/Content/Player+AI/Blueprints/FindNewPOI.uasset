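; FindNewPOI is a behavior tree task that picks a random point of interest for an OwnerAI pawn.
; It draws one entry from the pawn's POIArray as a POIBP and fails if that POI is in use or the pawn is not an OwnerAI.
; Otherwise it writes the POI to the CurrentPOIKey blackboard key, calls UseInteract on it and succeeds, with no retry on failure within the task.
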(event EventReceiveExecuteAI
  (params (OwnerController :type AI%20Controller%20Object%20Reference) (ControlledPawn :type Pawn%20Object%20Reference))
  (bind _asowner_ai (Utilities|Casting|CastToOwnerAI ControlledPawn)
    (:then
      (bind _new_poi (CallFunction|FindRandomObject (Variables|/Game/Player+AI/Blueprints/OwnerAI.OwnerAI_C|GetPOIArray _asowner_ai)))
      (bind _output_get (Variables|Default|SetCurrentActor _new_poi))
      (if (Variables|/Game/Blueprints/Other/POIBP.POIBP_C|GetinUse? _output_get)
        (AI|BehaviorTree|FinishExecute false)
        (else
          (AI|Components|Blackboard|SetValueasObject (AI|GetBlackboard ControlledPawn) (Variables|Default|GetCurrentPOIKey) _output_get)
          (Default|UseInteract (Variables|Default|GetCurrentActor))
          (AI|BehaviorTree|FinishExecute true))))
    (:CastFailed
      (AI|BehaviorTree|FinishExecute false))))

(fn FindRandomObject
  (params (ObjectArray :type Array%20of%20Actor%20Object%20References))
  (return (.AsPOIBP (Utilities|Casting|CastToPOIBP (Utilities|Array|Get(acopy) ObjectArray (Math|Random|RandomInteger (Utilities|Array|Length ObjectArray)))))))