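; Behavior tree task that walks an OwnerAI pawn through a UseableDoorBP stored under the blackboard's POI key.
; It calls UseInteract on the door, moves the pawn to the door's out-arrow then in-arrow location with short delays, then calls UseInteract again.
; It finishes successfully after that second interaction, and fails if either cast or move fails.
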(event EventReceiveExecuteAI
  (params (OwnerController :type AI%20Controller%20Object%20Reference) (ControlledPawn :type Pawn%20Object%20Reference))
  (Utilities|Casting|CastToOwnerAI ControlledPawn
    (:then
      (bind _asuseable_door_bp (Utilities|Casting|CastToUseableDoorBP (AI|BehaviorTree|GetBlackboardValueasActor (Variables|Default|GetPOIKey)))
        (:then
          (Default|UseInteract _asuseable_door_bp)
          (Utilities|FlowControl|Delay 0.5)
          (AI|AIMoveTo ControlledPawn (Variables|/Game/Blueprints/Interactables/UseableDoorBP.UseableDoorBP_C|GetOutArrowLocation _asuseable_door_bp) 0 1.0 false
            (:OnSuccess
              (Utilities|FlowControl|Delay 0.5)
              (AI|AIMoveTo ControlledPawn (Variables|/Game/Blueprints/Interactables/UseableDoorBP.UseableDoorBP_C|GetInArrowLocation _asuseable_door_bp) 0 1.0 false
                (:OnSuccess
                  (Default|UseInteract _asuseable_door_bp)
                  (AI|BehaviorTree|FinishExecute true))
                (:OnFail
                  (AI|BehaviorTree|FinishExecute false))))
            (:OnFail
              (AI|BehaviorTree|FinishExecute false))))
        (:CastFailed
          (AI|BehaviorTree|FinishExecute false))))
    (:CastFailed
      (AI|BehaviorTree|FinishExecute false))))