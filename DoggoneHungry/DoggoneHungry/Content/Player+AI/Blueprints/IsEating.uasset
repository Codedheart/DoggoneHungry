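; IsEating is a behavior tree decorator that passes when the AI has seen the player's dog and that dog is eating.
; It reads the seen flag and player object from the pawn's blackboard, then casts the object to BP_Dog to check IsEating.
; A check for the dog being up on furniture, based on mesh height, is left unconnected, so only eating counts.
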(fn PerformConditionCheckAI
  (params (OwnerController :type AI%20Controller%20Object%20Reference) (ControlledPawn :type Pawn%20Object%20Reference))
  (bind _returnvalue (AI|GetBlackboard ControlledPawn))
  (return (and (ScalableFloat|GetValueasBool _returnvalue (LocalVariables|GetisPlayerSeen_Key)) (or (Variables|/Game/Player+AI/Blueprints/BP_Dog.BP_Dog_C|GetisEating? (.AsBP%20Dog (Utilities|Casting|CastToBP_Dog (AI|Components|Blackboard|GetValueasObject _returnvalue (LocalVariables|GetPlayer_Key))))) false))))