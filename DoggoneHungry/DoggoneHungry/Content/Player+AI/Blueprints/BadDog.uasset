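; BadDog is a behavior tree task that plays the moment an OwnerAI or LifeGuardAI catches the player's dog.
; It switches the AI's animation state, shows a CaughtMessage widget and turns the BP_Dog camera, read from the blackboard, toward that AI.
; After a short delay it restores the animation state, deactivates the AI's particle, removes the widget and finishes successfully.
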(event EventReceiveExecuteAI
  (params (OwnerController :type AI%20Controller%20Object%20Reference) (ControlledPawn :type Pawn%20Object%20Reference))
  (bind _returnvalue (AI|GetBlackboard ControlledPawn))
  (bind _playerkey (Variables|Default|GetPlayerKey))
  (bind _returnvalue_2 (AI|Components|Blackboard|GetValueasObject _returnvalue _playerkey))
  (bind _asbp_dog (Utilities|Casting|CastToBP_Dog _returnvalue_2))
  (bind _asowner_ai (Utilities|Casting|CastToOwnerAI ControlledPawn)
    (:then
      (Variables|/Game/Player+AI/Blueprints/MasterAI.MasterAI_C|SetAnim%20State _asowner_ai "NewEnumerator7")
      (bind _returnvalue_3 (UserInterface|CreateWidget "/Game/UI/Widgets/CaughtMessage.CaughtMessage_C"))
      (bind _output_get (Variables|Default|SetCaughtMessage _returnvalue_3))
      (UserInterface|Viewport|AddtoViewport _output_get 0)
      (Default|RotateCameraTowardsEnemy _asbp_dog _asowner_ai)
      (Utilities|FlowControl|Delay 1.5)
      (Variables|/Game/Player+AI/Blueprints/MasterAI.MasterAI_C|SetAnim%20State _asowner_ai "NewEnumerator0")
      (Default|DeactivateParticle _asowner_ai)
      (Widget|RemovefromParent (Variables|Default|GetCaughtMessage))
      (AI|BehaviorTree|FinishExecute true))
    (:CastFailed
      (bind _aslife_guard_ai (Utilities|Casting|CastToLifeGuardAI ControlledPawn))
      (Variables|/Game/Player+AI/Blueprints/MasterAI.MasterAI_C|SetAnim%20State _aslife_guard_ai "NewEnumerator7")
      (bind _returnvalue_4 (UserInterface|CreateWidget "/Game/UI/Widgets/CaughtMessage.CaughtMessage_C"))
      (bind _output_get_2 (Variables|Default|SetCaughtMessage _returnvalue_4))
      (UserInterface|Viewport|AddtoViewport _output_get_2 0)
      (Default|RotateCameraTowardsEnemy _asbp_dog _aslife_guard_ai)
      (Utilities|FlowControl|Delay 1.5)
      (Variables|/Game/Player+AI/Blueprints/MasterAI.MasterAI_C|SetAnim%20State _aslife_guard_ai "NewEnumerator0")
      (Default|DeactivateParticle _aslife_guard_ai)
      (Widget|RemovefromParent (Variables|Default|GetCaughtMessage))
      (AI|BehaviorTree|FinishExecute true))))