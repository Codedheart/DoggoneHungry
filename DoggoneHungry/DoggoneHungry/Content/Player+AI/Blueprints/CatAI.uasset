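; Cat enemy that catches the player's dog when it moves too fast within the cat's view.
; A looping timer teleports it to a random CatSpawnPoint every few seconds.
; A second timer runs DetectionTrace, a pawn capsule overlap filtered by player speed and a horizontal dot-product angle check against DetectionDegree.
; A catch turns the dog's camera to the cat, shows particles and a message widget, then respawns the dog after a delay.
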(event Custom|CaughtDog!
  (bind _asbp_dog (Utilities|Casting|CastToBP_Dog (Game|GetPlayerCharacter 0)))
  (Default|RotateCameraTowardsEnemy _asbp_dog self)
  (Components|Activation|SetActive (Variables|Default|GetParticleSystem) true true)
  (Default|Caught _asbp_dog)
  (bind _returnvalue (UserInterface|CreateWidget "/Game/UI/Widgets/CaughtMessage.CaughtMessage_C" (Game|GetPlayerController 0)))
  (bind _output_get (Variables|Default|SetCaughtMessage _returnvalue))
  (UserInterface|Viewport|AddtoViewport _output_get 0)
  (Utilities|FlowControl|Delay 1.5)
  (Default|Respawn _asbp_dog)
  (Widget|RemovefromParent (Variables|Default|GetCaughtMessage))
  (Components|Activation|SetActive (Variables|Default|GetParticleSystem) false false))

(event Custom|SpawnRandomLocation
  (bind _spawnpoints (Variables|Default|GetSpawnPoints))
  (Transformation|SetActorTransform (Transformation|GetActorTransform (Utilities|Array|Get(acopy) _spawnpoints (Math|Random|RandomInteger (Utilities|Array|Length _spawnpoints)))) false true))

(event EventBeginPlay
  (Utilities|Time|SetTimerbyFunctionName 0 "DetectionTrace" 0.1 true)
  (bind _outactors (Actor|GetAllActorsOfClass "/Game/Blueprints/Other/CatSpawnPoint.CatSpawnPoint_C"))
  (Variables|Default|SetSpawnPoints _outactors)
  (Utilities|Time|SetTimerbyFunctionName 0 "SpawnRandomLocation" 5.0 true))

(fn ConstructionScript)

(fn DetectionTrace
  (bind _returnvalue (Transformation|GetActorLocation))
  (bind _returnvalue_2 (Transformation|GetActorForwardVector))
  (bind _returnvalue_3 (Transformation|GetActorLocation))
  (bind _returnvalue_4 (Game|Player|GetPlayerPawn 0))
  (bind _returnvalue_5 (Transformation|GetActorLocation _returnvalue_4))
  (bind _returnvalue_6 (Math|Vector|GetUnitDirection(Vector) _returnvalue_3 _returnvalue_5))
  (bind _outhits (Class|KismetSystemLibrary|CapsuleTraceMultiforObjects _returnvalue _returnvalue 3e+02 1e+03 (Utilities|Array|MakeArray "ObjectTypeQuery3") false (Utilities|Array|MakeArray self) "None" true))
  (for _array_element _outhits
    (if (== (.HitActor (Collision|BreakHitResult _array_element)) _returnvalue_4)
      (if (and (> (Math|Vector|VectorLength (Transformation|GetVelocity (Game|Player|GetPlayerPawn 0))) 301.0) (< (Class|KismetMathLibrary|DegAcos (Math|Vector|DotProduct (Math|Vector|MakeVector (.x _returnvalue_6) (.y _returnvalue_6) 0.0) (Math|Vector|MakeVector (.x _returnvalue_2) (.y _returnvalue_2) 0.0))) (Variables|Default|GetDetectionDegree)))
        (CallFunction|CaughtDog!)))))