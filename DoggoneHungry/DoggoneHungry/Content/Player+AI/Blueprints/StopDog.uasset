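; StopDog is a Behavior Tree task that lets an owner or lifeguard AI catch the player's dog.
; It reads the dog from the PlayerKey blackboard entry, calls Caught on it, triggers the catching pawn's particle effect and finishes successfully.
; OwnerAI and LifeGuardAI pawns run the same logic in separate cast branches, and a failed cast ends without calling FinishExecute.
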(event EventReceiveExecuteAI
  (params (OwnerController :type AI%20Controller%20Object%20Reference) (ControlledPawn :type Pawn%20Object%20Reference))
  (bind _playerkey (Variables|Default|GetPlayerKey))
  (bind _returnvalue (AI|BehaviorTree|GetBlackboardValueasActor _playerkey))
  (bind _asowner_ai (Utilities|Casting|CastToOwnerAI ControlledPawn)
    (:then
      (bind _asbp_dog (Utilities|Casting|CastToBP_Dog _returnvalue))
      (Default|Caught _asbp_dog 2.5)
      (Default|ActivateParticle _asowner_ai)
      (AI|BehaviorTree|FinishExecute true))
    (:CastFailed
      (bind _aslife_guard_ai (Utilities|Casting|CastToLifeGuardAI ControlledPawn))
      (bind _asbp_dog_2 (Utilities|Casting|CastToBP_Dog _returnvalue))
      (Default|Caught _asbp_dog_2 2.5)
      (Default|ActivateParticle _aslife_guard_ai)
      (AI|BehaviorTree|FinishExecute true))))