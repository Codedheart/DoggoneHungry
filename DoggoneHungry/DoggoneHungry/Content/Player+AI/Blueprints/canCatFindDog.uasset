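; Behavior tree decorator that, going by its name, gates whether the cat AI can find the player's dog.
; It reads the Player blackboard object as BP_Dog and checks whether the dog is acting or moving faster than a fixed speed threshold.
; The condition passes only when either of those holds and the IsPlayerSeen blackboard flag is also true.
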(fn PerformConditionCheckAI
  (params (OwnerController :type AI%20Controller%20Object%20Reference) (ControlledPawn :type Pawn%20Object%20Reference))
  (bind _player (Variables|Default|GetPlayer))
  (bind _returnvalue (Class|BTFunctionLibrary|GetBlackboardValueasObject _player))
  (bind _asbp_dog (Utilities|Casting|CastToBP_Dog _returnvalue))
  (return (and (or (Variables|/Game/Player+AI/Blueprints/BP_Dog.BP_Dog_C|GetisActing? _asbp_dog) (> (Math|Vector|VectorLength (Transformation|GetVelocity _asbp_dog)) 301.0)) (Class|BTFunctionLibrary|GetBlackboardValueasBool (Variables|Default|GetisPlayerSeen?)))))