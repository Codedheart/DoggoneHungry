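; Behavior tree task that looks for a nearby bark point of interest for the AI-controlled pawn.
; It runs a multi sphere trace from the pawn along its up vector and collects hit actors carrying the bark POI tag.
; If the first is a UseableDoorBP, it stores it in the blackboard as the interactable object.
; The task succeeds whenever the trace reports a hit, even without a matching door, and fails otherwise.
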(event EventReceiveExecuteAI
  (params (OwnerController :type AI%20Controller%20Object%20Reference) (ControlledPawn :type Pawn%20Object%20Reference))
  (bind _returnvalue (Transformation|GetActorLocation ControlledPawn))
  (Utilities|Array|Clear (Variables|Default|GetHitActors))
  (bind (_outhits _returnvalue_2) (Collision|MultiSphereTraceByChannel _returnvalue (+ _returnvalue (* (Transformation|GetActorUpVector ControlledPawn) (Variables|Default|GetTraceDistance))) (Variables|Default|GetRadius) "TraceTypeQuery1" false 0 "None"))
  (if _returnvalue_2
    (bind _array_element (Utilities|Array|ForEachLoopwithBreak _outhits)
      (:LoopBody
        (if (Actor|ActorHasTag (.HitActor (Collision|BreakHitResult _array_element)) (Variables|Default|GetBarkPOIKey))
          (Utilities|Array|Add (Variables|Default|GetHitActors) (.HitActor (Collision|BreakHitResult _array_element)))))
      (:Completed
        (bind _asuseable_door_bp (Utilities|Casting|CastToUseableDoorBP (Utilities|Array|Get(acopy) (Variables|Default|GetHitActors)))
          (:then
            (AI|Components|Blackboard|SetValueasObject (AI|GetBlackboard ControlledPawn) (Variables|Default|GetInteractableObjectKey) _asuseable_door_bp))
          (:CastFailed
            _))
        (AI|BehaviorTree|FinishExecute true)))
    (else
      (AI|BehaviorTree|FinishExecute false))))