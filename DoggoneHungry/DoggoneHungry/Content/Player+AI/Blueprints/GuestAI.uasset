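; Guest NPC that the player dog interacts with to start a minigame if the dog meets the guest's attribute requirement.
; UseInteract compares the blackboard player's matching stat to a threshold and checks TricksDone, then plays approval or rejection feedback.
; A widget shows the requirement when toggled visible, and a looping timer turns its scene component toward the dog's camera.
; The tutorial level effectively lifts the trick limit, and a rejection there can advance the tutorial task.
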(event Custom|InformationRotation
  (bind _scene (Variables|Default|GetScene))
  (bind _asbp_dog (Utilities|Casting|CastToBP_Dog (Game|GetPlayerCharacter 0)))
  (Transformation|SetWorldRotation _scene (Math|Rotator|FindLookatRotation (Transformation|GetWorldLocation _scene) (Transformation|GetWorldLocation (Variables|/Game/Player+AI/Blueprints/BP_Dog.BP_Dog_C|GetFollowCamera _asbp_dog))) false false))

(event Custom|HideWidget
  ;[1 1 1] Display NPC Information if NPC is Highlighted
  (Rendering|SetVisibility (Variables|Default|GetInformationDisplay) false false))

(event Custom|ShowWidget
  ;[1 1 1] Display NPC Information if NPC is Highlighted
  (Rendering|SetVisibility (Variables|Default|GetInformationDisplay) true false))

(event Custom|SpawnNPC)

(event EventBeginPlay
  (Utilities|Time|SetTimerbyFunctionName 0 "InformationRotation" 0.01 true)
  ;[1 1 1] Construct NPC Information Widget
  (bind _asnpcinformation_display (Utilities|Casting|CastToNPCInformationDisplay (UserInterface|GetUserWidgetObject (Variables|Default|GetInformationDisplay))))
  (Variables|/Game/UI/Widgets/NPCInformationDisplay.NPCInformationDisplay_C|SetAttributeEnum _asnpcinformation_display (Variables|AttributeToCheck|GetAttributeCheckEnum))
  (Variables|/Game/UI/Widgets/NPCInformationDisplay.NPCInformationDisplay_C|SetDifficulty _asnpcinformation_display (Variables|AttributetoCheck|GetBasePassingValue))
  (bind _returnvalue (Game|GetCurrentLevelName true))
  (if (Utilities|Enum|Equal(Enum) _returnvalue "Tutorial_Level")
    (Variables|Default|SetTricksDone -99999)))

(event EventTick
  (params (DeltaSeconds :type Float%20%28single-precision%29)))

(event EventUseInteract
  (params (UsingActor :type Actor%20Object%20Reference))
  ;[1 1 1] Start a minigame if we meet the requirements
  (bind _asbp_dog (Utilities|Casting|CastToBP_Dog UsingActor))
  (bind _passedcheck_ (CallFunction|CheckPlayerAttributes))
  (if (and _passedcheck_ (<= (Variables|Default|GetTricksDone) 1))
    (Variables|Default|SetAnim%20State "NewEnumerator5")
    (Audio|PlaySound2D "/Game/Sound/ABS/ABS_Approval_MiniGameStart.ABS_Approval_MiniGameStart" 1.0 1.0 0.0 0 0)
    (Utilities|FlowControl|Delay 1.0)
    (if (Variables|/Game/Player+AI/Blueprints/BP_Dog.BP_Dog_C|GetbTutorialLevel _asbp_dog)
      (Game|Player|SetViewTargetwithBlend (Game|GetPlayerController 0) _asbp_dog 0.1 "VTBlend_Linear" 0.0 false)
      (Default|ChooseRandomMinigame _asbp_dog 0)
      (else
        (Default|ChooseRandomMinigame _asbp_dog -1)))
    (else
      (Variables|Default|SetAnim%20State "NewEnumerator8")
      (Audio|PlaySound2D "/Game/Sound/ABS/ABS_Rejected.ABS_Rejected" 1.0 1.0 0.0 0 0)
      (if (Variables|/Game/Player+AI/Blueprints/BP_Dog.BP_Dog_C|GetbTutorialLevel _asbp_dog)
        (Utilities|FlowControl|DoOnce false
          (:Completed
            (Default|NextTaskforTutorial (Variables|/Game/Player+AI/Blueprints/BP_Dog.BP_Dog_C|GetTutorialController _asbp_dog))))))))

(fn ConstructionScript
  (|CallParentFunction))

(fn CheckPlayerAttributes
  (bind _returnvalue (AI|GetBlackboard 0))
  (bind _playerkey (Variables|Default|GetPlayerKey))
  (bind _returnvalue_2 (AI|Components|Blackboard|GetValueasObject _returnvalue _playerkey))
  (bind _asbp_dog (Utilities|Casting|CastToBP_Dog _returnvalue_2))
  (bind _playerstats (Variables|/Game/Player+AI/Blueprints/BP_Dog.BP_Dog_C|GetPlayerStats _asbp_dog))
  (switch Utilities|FlowControl|Switch|SwitchonAttributeCheckEnum (Variables|AttributeToCheck|GetAttributeCheckEnum)
    (:NewEnumerator0
      (LocalVariables|SetAttributeValue (.fancyness _playerstats)))
    (:NewEnumerator1
      (LocalVariables|SetAttributeValue (.stinkiness _playerstats)))
    (:NewEnumerator2
      (LocalVariables|SetAttributeValue (.cuteness _playerstats)))
    (:NewEnumerator3
      (LocalVariables|SetAttributeValue (.wackiness _playerstats)))
    (:NewEnumerator4
      (LocalVariables|SetAttributeValue (.coolness _playerstats))))
  (return (>= (LocalVariables|GetAttributeValue) (Variables|AttributetoCheck|GetBasePassingValue))))