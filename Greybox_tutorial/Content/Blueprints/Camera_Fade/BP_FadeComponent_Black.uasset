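; Actor component for camera fade that hides a Static Mesh Actor by swapping its materials for a fade material.
; BeginPlay caches the materials in a fixed run of slots, stopping at the first failed Material cast, and creates a dynamic instance of FadeMaterial.
; ToggleHideMesh applies that instance to the slots when switched to hidden.
; Tick restores cached materials while unhidden and CurrentFade equals one; nothing here animates that value.
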(event EventBeginPlay
  ;[1 1 1] Setup Component
  (bind _asstatic_mesh_actor (Utilities|Casting|CastToStaticMeshActor (Components|GetOwner))) ; Get Static Mesh Actor
  (bind _output_get (Variables|Default|SetParrentMesh _asstatic_mesh_actor))
  (bind _asmaterial (Utilities|Casting|CastToMaterial (Utilities|Array|Get(acopy) (Rendering|Material|GetMaterials (Variables|/Script/Engine.StaticMeshActor|GetStaticMeshComponent _output_get)))))
  (Variables|Default|SetBaseMaterial _asmaterial)
  (bind _returnvalue (Rendering|Material|CreateDynamicMaterialInstance (Variables|Default|GetFadeMaterial) "None" :!class /Script/Engine.KismetMaterialLibrary))
  (Variables|Default|SetFadeMaterialMID _returnvalue)
  (bind _asmaterial_2 (Utilities|Casting|CastToMaterial (Utilities|Array|Get(acopy) (Rendering|Material|GetMaterials (Variables|/Script/Engine.StaticMeshActor|GetStaticMeshComponent _output_get)) 1)))
  (Variables|Default|SetBaseMaterial_0 _asmaterial_2)
  (bind _asmaterial_3 (Utilities|Casting|CastToMaterial (Utilities|Array|Get(acopy) (Rendering|Material|GetMaterials (Variables|/Script/Engine.StaticMeshActor|GetStaticMeshComponent _output_get)) 2)))
  (Variables|Default|SetBaseMaterial_1 _asmaterial_3)
  (bind _asmaterial_4 (Utilities|Casting|CastToMaterial (Utilities|Array|Get(acopy) (Rendering|Material|GetMaterials (Variables|/Script/Engine.StaticMeshActor|GetStaticMeshComponent _output_get)) 3)))
  (Variables|Default|SetBaseMaterial_2 _asmaterial_4)
  (bind _asmaterial_5 (Utilities|Casting|CastToMaterial (Utilities|Array|Get(acopy) (Rendering|Material|GetMaterials (Variables|/Script/Engine.StaticMeshActor|GetStaticMeshComponent _output_get)) 4)))
  (Variables|Default|SetBaseMaterial_3 _asmaterial_5)
  (bind _asmaterial_6 (Utilities|Casting|CastToMaterial (Utilities|Array|Get(acopy) (Rendering|Material|GetMaterials (Variables|/Script/Engine.StaticMeshActor|GetStaticMeshComponent _output_get)) 5)))
  (Variables|Default|SetBaseMaterial_4 _asmaterial_6)
  (bind _asmaterial_7 (Utilities|Casting|CastToMaterial (Utilities|Array|Get(acopy) (Rendering|Material|GetMaterials (Variables|/Script/Engine.StaticMeshActor|GetStaticMeshComponent _output_get)) 6)))
  (Variables|Default|SetBaseMaterial_5 _asmaterial_7)
  (bind _asmaterial_8 (Utilities|Casting|CastToMaterial (Utilities|Array|Get(acopy) (Rendering|Material|GetMaterials (Variables|/Script/Engine.StaticMeshActor|GetStaticMeshComponent _output_get)) 7)))
  (Variables|Default|SetBaseMaterial_6 _asmaterial_8)
  (bind _asmaterial_9 (Utilities|Casting|CastToMaterial (Utilities|Array|Get(acopy) (Rendering|Material|GetMaterials (Variables|/Script/Engine.StaticMeshActor|GetStaticMeshComponent _output_get)) 8)))
  (Variables|Default|SetBaseMaterial_7 _asmaterial_9)
  (bind _asmaterial_10 (Utilities|Casting|CastToMaterial (Utilities|Array|Get(acopy) (Rendering|Material|GetMaterials (Variables|/Script/Engine.StaticMeshActor|GetStaticMeshComponent _output_get)) 9)))
  (Variables|Default|SetBaseMaterial_8 _asmaterial_10)
  (bind _asmaterial_11 (Utilities|Casting|CastToMaterial (Utilities|Array|Get(acopy) (Rendering|Material|GetMaterials (Variables|/Script/Engine.StaticMeshActor|GetStaticMeshComponent _output_get)) 10)))
  (Variables|Default|SetBaseMaterial_9 _asmaterial_11)
  (bind _asmaterial_12 (Utilities|Casting|CastToMaterial (Utilities|Array|Get(acopy) (Rendering|Material|GetMaterials (Variables|/Script/Engine.StaticMeshActor|GetStaticMeshComponent _output_get)) 11)))
  (Variables|Default|SetBaseMaterial_10 _asmaterial_12)
  (bind _asmaterial_13 (Utilities|Casting|CastToMaterial (Utilities|Array|Get(acopy) (Rendering|Material|GetMaterials (Variables|/Script/Engine.StaticMeshActor|GetStaticMeshComponent _output_get)) 12)))
  (Variables|Default|SetBaseMaterial_11 _asmaterial_13)
  (bind _asmaterial_14 (Utilities|Casting|CastToMaterial (Utilities|Array|Get(acopy) (Rendering|Material|GetMaterials (Variables|/Script/Engine.StaticMeshActor|GetStaticMeshComponent _output_get)) 13)))
  (Variables|Default|SetBaseMaterial_12 _asmaterial_14)
  (bind _asmaterial_15 (Utilities|Casting|CastToMaterial (Utilities|Array|Get(acopy) (Rendering|Material|GetMaterials (Variables|/Script/Engine.StaticMeshActor|GetStaticMeshComponent _output_get)) 14)))
  (Variables|Default|SetBaseMaterial_13 _asmaterial_15)
  (bind _asmaterial_16 (Utilities|Casting|CastToMaterial (Utilities|Array|Get(acopy) (Rendering|Material|GetMaterials (Variables|/Script/Engine.StaticMeshActor|GetStaticMeshComponent _output_get)) 15)))
  (Variables|Default|SetBaseMaterial_14 _asmaterial_16)
  (bind _asmaterial_17 (Utilities|Casting|CastToMaterial (Utilities|Array|Get(acopy) (Rendering|Material|GetMaterials (Variables|/Script/Engine.StaticMeshActor|GetStaticMeshComponent _output_get)) 16)))
  (Variables|Default|SetBaseMaterial_15 _asmaterial_17)
  (bind _asmaterial_18 (Utilities|Casting|CastToMaterial (Utilities|Array|Get(acopy) (Rendering|Material|GetMaterials (Variables|/Script/Engine.StaticMeshActor|GetStaticMeshComponent _output_get)) 17)))
  (Variables|Default|SetBaseMaterial_16 _asmaterial_18)
  (bind _asmaterial_19 (Utilities|Casting|CastToMaterial (Utilities|Array|Get(acopy) (Rendering|Material|GetMaterials (Variables|/Script/Engine.StaticMeshActor|GetStaticMeshComponent _output_get)) 18)))
  (Variables|Default|SetBaseMaterial_17 _asmaterial_19))

(event EventTick
  (params (DeltaSeconds :type Float%20%28single-precision%29))
  ;[1 1 1] Fade over time
  (Utilities|IsValid (Variables|Default|GetParrentMesh)
    (:Is%20Valid
      (if (and (== (Variables|Default|GetCurrentFade) 1.0) (not (Variables|Default|GetHidden)))
        (Rendering|Material|SetMaterial (Variables|/Script/Engine.StaticMeshActor|GetStaticMeshComponent (Variables|Default|GetParrentMesh)) 0 (Variables|Default|GetBaseMaterial))
        (Rendering|Material|SetMaterial (Variables|/Script/Engine.StaticMeshActor|GetStaticMeshComponent (Variables|Default|GetParrentMesh)) 1 (Variables|Default|GetBaseMaterial_0))
        (Rendering|Material|SetMaterial (Variables|/Script/Engine.StaticMeshActor|GetStaticMeshComponent (Variables|Default|GetParrentMesh)) 2 (Variables|Default|GetBaseMaterial_1))
        (Rendering|Material|SetMaterial (Variables|/Script/Engine.StaticMeshActor|GetStaticMeshComponent (Variables|Default|GetParrentMesh)) 3 (Variables|Default|GetBaseMaterial_2))
        (Rendering|Material|SetMaterial (Variables|/Script/Engine.StaticMeshActor|GetStaticMeshComponent (Variables|Default|GetParrentMesh)) 4 (Variables|Default|GetBaseMaterial_3))
        (Rendering|Material|SetMaterial (Variables|/Script/Engine.StaticMeshActor|GetStaticMeshComponent (Variables|Default|GetParrentMesh)) 5 (Variables|Default|GetBaseMaterial_4))
        (Rendering|Material|SetMaterial (Variables|/Script/Engine.StaticMeshActor|GetStaticMeshComponent (Variables|Default|GetParrentMesh)) 6 (Variables|Default|GetBaseMaterial_5))
        (Rendering|Material|SetMaterial (Variables|/Script/Engine.StaticMeshActor|GetStaticMeshComponent (Variables|Default|GetParrentMesh)) 7 (Variables|Default|GetBaseMaterial_6))
        (Rendering|Material|SetMaterial (Variables|/Script/Engine.StaticMeshActor|GetStaticMeshComponent (Variables|Default|GetParrentMesh)) 8 (Variables|Default|GetBaseMaterial_7))
        (Rendering|Material|SetMaterial (Variables|/Script/Engine.StaticMeshActor|GetStaticMeshComponent (Variables|Default|GetParrentMesh)) 9 (Variables|Default|GetBaseMaterial_8))
        (Rendering|Material|SetMaterial (Variables|/Script/Engine.StaticMeshActor|GetStaticMeshComponent (Variables|Default|GetParrentMesh)) 10 (Variables|Default|GetBaseMaterial_9))
        (Rendering|Material|SetMaterial (Variables|/Script/Engine.StaticMeshActor|GetStaticMeshComponent (Variables|Default|GetParrentMesh)) 11 (Variables|Default|GetBaseMaterial_10))
        (Rendering|Material|SetMaterial (Variables|/Script/Engine.StaticMeshActor|GetStaticMeshComponent (Variables|Default|GetParrentMesh)) 12 (Variables|Default|GetBaseMaterial_11))
        (Rendering|Material|SetMaterial (Variables|/Script/Engine.StaticMeshActor|GetStaticMeshComponent (Variables|Default|GetParrentMesh)) 13 (Variables|Default|GetBaseMaterial_12))
        (Rendering|Material|SetMaterial (Variables|/Script/Engine.StaticMeshActor|GetStaticMeshComponent (Variables|Default|GetParrentMesh)) 14 (Variables|Default|GetBaseMaterial_13))
        (Rendering|Material|SetMaterial (Variables|/Script/Engine.StaticMeshActor|GetStaticMeshComponent (Variables|Default|GetParrentMesh)) 15 (Variables|Default|GetBaseMaterial_14))
        (Rendering|Material|SetMaterial (Variables|/Script/Engine.StaticMeshActor|GetStaticMeshComponent (Variables|Default|GetParrentMesh)) 16 (Variables|Default|GetBaseMaterial_15))
        (Rendering|Material|SetMaterial (Variables|/Script/Engine.StaticMeshActor|GetStaticMeshComponent (Variables|Default|GetParrentMesh)) 17 (Variables|Default|GetBaseMaterial_16))
        (Rendering|Material|SetMaterial (Variables|/Script/Engine.StaticMeshActor|GetStaticMeshComponent (Variables|Default|GetParrentMesh)) 18 (Variables|Default|GetBaseMaterial_17))
        (Rendering|Material|SetMaterial (Variables|/Script/Engine.StaticMeshActor|GetStaticMeshComponent (Variables|Default|GetParrentMesh)) 19 (Variables|Default|GetBaseMaterial_18))))))

(fn ToggleHideMesh
  (params (Hidden :type Boolean))
  (bind _fadematerialmid (Variables|Default|GetFadeMaterialMID))
  ;[1 1 1] Toggle hidden / show
  (if (Math|Boolean|NotEqual(Boolean) Hidden (Variables|Default|GetHidden)) ; Only if Changing
    (bind _output_get (Variables|Default|SetHidden Hidden))
    (if _output_get ; True = Hidden
      (Rendering|Material|SetMaterial (Variables|/Script/Engine.StaticMeshActor|GetStaticMeshComponent (Variables|Default|GetParrentMesh)) 0 _fadematerialmid)
      (Rendering|Material|SetMaterial (Variables|/Script/Engine.StaticMeshActor|GetStaticMeshComponent (Variables|Default|GetParrentMesh)) 1 _fadematerialmid)
      (Rendering|Material|SetMaterial (Variables|/Script/Engine.StaticMeshActor|GetStaticMeshComponent (Variables|Default|GetParrentMesh)) 2 _fadematerialmid)
      (Rendering|Material|SetMaterial (Variables|/Script/Engine.StaticMeshActor|GetStaticMeshComponent (Variables|Default|GetParrentMesh)) 3 _fadematerialmid)
      (Rendering|Material|SetMaterial (Variables|/Script/Engine.StaticMeshActor|GetStaticMeshComponent (Variables|Default|GetParrentMesh)) 4 _fadematerialmid)
      (Rendering|Material|SetMaterial (Variables|/Script/Engine.StaticMeshActor|GetStaticMeshComponent (Variables|Default|GetParrentMesh)) 5 _fadematerialmid)
      (Rendering|Material|SetMaterial (Variables|/Script/Engine.StaticMeshActor|GetStaticMeshComponent (Variables|Default|GetParrentMesh)) 6 _fadematerialmid)
      (Rendering|Material|SetMaterial (Variables|/Script/Engine.StaticMeshActor|GetStaticMeshComponent (Variables|Default|GetParrentMesh)) 7 _fadematerialmid)
      (Rendering|Material|SetMaterial (Variables|/Script/Engine.StaticMeshActor|GetStaticMeshComponent (Variables|Default|GetParrentMesh)) 8 _fadematerialmid)
      (Rendering|Material|SetMaterial (Variables|/Script/Engine.StaticMeshActor|GetStaticMeshComponent (Variables|Default|GetParrentMesh)) 9 _fadematerialmid)
      (Rendering|Material|SetMaterial (Variables|/Script/Engine.StaticMeshActor|GetStaticMeshComponent (Variables|Default|GetParrentMesh)) 10 _fadematerialmid)
      (Rendering|Material|SetMaterial (Variables|/Script/Engine.StaticMeshActor|GetStaticMeshComponent (Variables|Default|GetParrentMesh)) 11 _fadematerialmid)
      (Rendering|Material|SetMaterial (Variables|/Script/Engine.StaticMeshActor|GetStaticMeshComponent (Variables|Default|GetParrentMesh)) 12 _fadematerialmid)
      (Rendering|Material|SetMaterial (Variables|/Script/Engine.StaticMeshActor|GetStaticMeshComponent (Variables|Default|GetParrentMesh)) 13 _fadematerialmid)
      (Rendering|Material|SetMaterial (Variables|/Script/Engine.StaticMeshActor|GetStaticMeshComponent (Variables|Default|GetParrentMesh)) 14 _fadematerialmid)
      (Rendering|Material|SetMaterial (Variables|/Script/Engine.StaticMeshActor|GetStaticMeshComponent (Variables|Default|GetParrentMesh)) 15 _fadematerialmid)
      (Rendering|Material|SetMaterial (Variables|/Script/Engine.StaticMeshActor|GetStaticMeshComponent (Variables|Default|GetParrentMesh)) 16 _fadematerialmid)
      (Rendering|Material|SetMaterial (Variables|/Script/Engine.StaticMeshActor|GetStaticMeshComponent (Variables|Default|GetParrentMesh)) 17 _fadematerialmid)
      (Rendering|Material|SetMaterial (Variables|/Script/Engine.StaticMeshActor|GetStaticMeshComponent (Variables|Default|GetParrentMesh)) 18 _fadematerialmid))))