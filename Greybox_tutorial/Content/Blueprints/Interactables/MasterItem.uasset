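; MasterItem is an interactable item actor, apparently a base for pickups, with an ItemInfo struct and a floating widget for the BP_Dog player.
; Each tick, Scene turns toward the dog's follow camera and is repositioned a fixed height above the static mesh, keeping the widget readable.
; The construction script fills ItemInfo with a self reference and the current mesh.
; Interacting destroys the actor, while the show and hide widget events are empty.
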(event Custom|ShowWidget)

(event Custom|HideWidget)

(event EventTick
  (params (DeltaSeconds :type Float%20%28single-precision%29))
  (bind _staticmesh (Variables|Default|GetStaticMesh))
  (bind _scene (Variables|Default|GetScene))
  (bind _returnvalue (Transformation|GetWorldLocation _staticmesh))
  ;[1 1 1] Widget will always face player camera
  (bind _asbp_dog (Utilities|Casting|CastToBP_Dog (Game|GetPlayerCharacter 0)))
  (Transformation|SetWorldRotation _scene (Math|Rotator|FindLookatRotation (Transformation|GetWorldLocation _scene) (Transformation|GetWorldLocation (Variables|/Game/Player+AI/Blueprints/BP_Dog.BP_Dog_C|GetFollowCamera _asbp_dog))) false false)
  ;[1 1 1] Get widget to always display directly above item
  (Transformation|SetWorldLocation _scene (Math|Vector|MakeVector (.x _returnvalue) (.y _returnvalue) (+ (.z _returnvalue) 82.0)) false false))

(event EventUseInteract
  (params (UsingActor :type Actor%20Object%20Reference))
  (Actor|DestroyActor))

(fn ConstructionScript
  (Variables|Default|SetItemInfo (Utilities|Struct|MakeEquippableItemInfo (.skeletalmesh (Variables|Default|GetItemInfo)) self (.slotname (Variables|Default|GetItemInfo)) (.attributeenum (Variables|Default|GetItemInfo)) (Variables|/Script/Engine.StaticMeshComponent|GetStaticMesh (Variables|Default|GetStaticMesh)) (.name (Variables|Default|GetItemInfo)) (.value (Variables|Default|GetItemInfo)))) ; Automatically set a reference to self
)