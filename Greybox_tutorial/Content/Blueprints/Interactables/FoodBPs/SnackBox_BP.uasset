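; SnackBox_BP is an interactable food item that shows its name on a widget component.
; On BeginPlay it sets the ObjectInformationDisplay widget's text from ItemInfo.Name and removes the display image from that widget.
; ShowWidget and HideWidget events toggle the widget's visibility, and the construction script only calls its parent.
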(event EventBeginPlay
  (bind _asobject_information_display (Utilities|Casting|CastToObjectInformationDisplay (UserInterface|GetUserWidgetObject (Variables|Default|GetWidget))))
  (Variables|/Game/UI/Widgets/ObjectInformationDisplay.ObjectInformationDisplay_C|SetDisplayText _asobject_information_display (.name (Variables|Default|GetItemInfo)))
  (Widget|RemovefromParent (Variables|/Game/UI/Widgets/ObjectInformationDisplay.ObjectInformationDisplay_C|GetDisplayImage _asobject_information_display)))

(event EventShowWidget
  (Rendering|SetVisibility (Variables|Default|GetWidget) true false))

(event EventHideWidget
  (Rendering|SetVisibility (Variables|Default|GetWidget) false false))

(fn ConstructionScript
  (|CallParentFunction))