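; WinTree is the level's win trigger, an interactable with a toy attached that ends the game when the _00 actor reaches it fully morphed.
; Its Sphere overlap checks that the actor's CurrentMorphTargetValue is at least 1, then fires once.
; It swaps the Toy component for a spawned DogToy_BP at the same transform, then opens Win_Level after a short delay.
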(event OnComponentBeginOverlap(Sphere)
  (params (OverlappedComponent :type Primitive%20Component%20Object%20Reference) (OtherActor :type Actor%20Object%20Reference) (OtherComp :type Primitive%20Component%20Object%20Reference) (OtherBodyIndex :type Integer) (bFromSweep :type Boolean) (SweepResult :type Hit%20Result%20Structure%20%28by%20ref%29))
  (bind _toy (Variables|Default|GetToy))
  (bind _as_00 (Utilities|Casting|CastTo_00 OtherActor))
  (if (>= (Variables|/Game/Player+AI/Blueprints/_00._00_C|GetCurrentMorphTargetValue _as_00) 1.0)
    (Utilities|FlowControl|DoOnce false
      (:Completed
        (Game|SpawnActorfromClass "/Game/Blueprints/Other/DogToy_BP.DogToy_BP_C" (Transformation|GetWorldTransform _toy) "Undefined" 0 0)
        (Components|DestroyComponent _toy)
        (Utilities|FlowControl|Delay 2.5)
        (Game|OpenLevel(byName) "Win_Level")))))

(fn ConstructionScript)