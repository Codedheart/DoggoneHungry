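; RecordingActor_Player is an actor that spins continuously and exposes dog-trick style states: sit, beg, roll over and play dead.
; Tick yaws the Scene component by a fixed step each frame, so spin speed depends on frame rate.
; Each trick event restarts a shared timer, clears all state flags and sets its own, keeping tricks mutually exclusive until CancelAnimations resets them when the timer expires.
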(event Custom|Sit
  (CallFunction|AnimTimer 3.0)
  (CallFunction|CancelAnimations)
  (Variables|Default|SetisSitting true))

(event Custom|Beg
  (CallFunction|AnimTimer 3.0)
  (CallFunction|CancelAnimations)
  (Variables|Default|SetisBegging true))

(event Custom|Roll%20Over
  (CallFunction|AnimTimer 3.0)
  (CallFunction|CancelAnimations)
  (Variables|Default|SetisRollingOver true))

(event Custom|Play%20Dead
  (CallFunction|AnimTimer 3.0)
  (CallFunction|CancelAnimations)
  (Variables|Default|SetisPlayingDead true))

(event EventTick
  (params (DeltaSeconds :type Float%20%28single-precision%29))
  (bind _scene (Variables|Default|GetScene))
  (bind _returnvalue (Transformation|GetWorldRotation _scene))
  (Transformation|SetWorldRotation _scene (Math|Rotator|MakeRotator (.roll _returnvalue) (.pitch _returnvalue) (+ (.yaw _returnvalue) 1.0)) false false))

(fn ConstructionScript)

(fn CancelAnimations
  (Variables|Default|SetisPlayingDead false)
  (Variables|Default|SetisRollingOver false)
  (Variables|Default|SetisBegging false)
  (Variables|Default|SetisSitting false))

(fn AnimTimer
  (params (Time :type Float%20%28single-precision%29))
  (Utilities|Time|ClearandInvalidateTimerbyHandle (stale _returnvalue))
  (bind _returnvalue (Utilities|Time|SetTimerbyFunctionName 0 "CancelAnimations" Time)))