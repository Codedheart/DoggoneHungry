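; BP_BalancedFood is a food actor that stays balanced while attached and drops as a physics object when balance fails.
; Every Tick resets the actor's rotation to a fixed default with physics teleport, with no check for whether it has fallen.
; FailBalance detaches it keeping its world transform, switches the static mesh to physics-only collision and simulation, then pushes it along the mesh's forward vector.
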(event Custom|FailBalance
  (bind _staticmesh (Variables|Default|GetStaticMesh))
  (Transformation|DetachFromActor "KeepWorld" "KeepWorld" "KeepWorld")
  (Collision|SetCollisionEnabled _staticmesh "PhysicsOnly")
  (Physics|SetSimulatePhysics _staticmesh true)
  (Physics|AddForce _staticmesh (* (Math|Vector|GetForwardVector _staticmesh) 5e+02) "None" false))

(event EventBeginPlay)

(event Collision|EventActorBeginOverlap
  (params (OtherActor :type Actor%20Object%20Reference)))

(event EventTick
  (params (DeltaSeconds :type Float%20%28single-precision%29))
  (Transformation|SetActorRotation (Math|Rotator|MakeRotator 0.0 0.0 0.0) true))

(fn ConstructionScript)