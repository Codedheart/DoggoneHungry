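; Basic AI controller that starts the BT_Owner behavior tree on BeginPlay and seeds its blackboard with a player target.
; It gathers all actors of class _00 into PlayerArray and writes the first one to PlayerKey and its location to LocationKey.
; The location is a one-time snapshot with no later updates here, and an empty search only prints a debug message.
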(event EventBeginPlay
  (AI|RunBehaviorTree "/Game/Player+AI/Blueprints/BT_Owner.BT_Owner")
  (bind _outactors (Actor|GetAllActorsOfClass "/Game/Player+AI/Blueprints/_00._00_C"))
  (bind _output_get (Variables|Default|SetPlayerArray _outactors))
  (if (> (Utilities|Array|Length _output_get) 0)
    (AI|Components|Blackboard|SetValueasObject (AI|GetBlackboard 0) (Variables|Default|GetPlayer_Key) (Utilities|Array|Get(acopy) _output_get))
    (AI|Components|Blackboard|SetValueasVector (AI|GetBlackboard 0) (Variables|Default|GetLocation_Key) (Transformation|GetActorLocation (Utilities|Array|Get(acopy) _output_get)))
    (else
      (Development|PrintString "NO ACTORS FOUND"))))

(fn ConstructionScript)