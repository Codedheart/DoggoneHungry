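; Party guest NPC that starts a random minigame when the dog player interacts with enough of its required attribute and few tricks done, otherwise rejects them.
; On BeginPlay it gathers other guests, seeds the Blackboard and starts a one-shot bathroom timer.
; The timer and conversation events set Blackboard keys for AI behavior.
; An information widget shows the required attribute and difficulty, while Tick turns a scene component toward the player camera.
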(event Custom|NeedToGO
  (AI|Components|Blackboard|SetValueasBool (AI|GetBlackboard 0) (Variables|Default|GetBathroomKey) true))

(event Custom|StartBathroomTimer
  (bind _returnvalue (Utilities|Time|SetTimerbyEvent (delegate Custom|NeedToGO) (Variables|Default|GetBathroomTimer)))
  (Variables|Default|SetTimer _returnvalue))

(event Custom|ShowWidget
  (Rendering|SetVisibility (Variables|Default|GetInformationDisplay) true false))

(event Custom|HideWidget
  (Rendering|SetVisibility (Variables|Default|GetInformationDisplay) false false))

(event EventBeginPlay
  (bind _returnvalue (AI|GetBlackboard 0))
  (AI|Components|Blackboard|SetValueasObject _returnvalue (Variables|Default|GetConversationCueKey) 0)
  (AI|Components|Blackboard|SetValueasVector _returnvalue (Variables|Default|GetInitialLocation) (Transformation|GetActorLocation))
  (CallFunction|StartBathroomTimer)
  (bind _outactors (Actor|GetAllActorsOfClass "GuestAI_C"))
  (for _array_element _outactors
    (if (not (== _array_element self))
      (Utilities|Array|Add (Variables|Default|GetGuestArray) _array_element)))
  ;[1 1 1] Construct NPC Information Widget
  (bind _asnpcinformation_display (Utilities|Casting|CastToNPCInformationDisplay (UserInterface|GetUserWidgetObject (Variables|Default|GetInformationDisplay))))
  (Variables|/Game/UI/Widgets/NPCInformationDisplay.NPCInformationDisplay_C|SetAttributeEnum _asnpcinformation_display (Variables|AttributeToCheck|GetAttributeCheckEnum))
  (Variables|/Game/UI/Widgets/NPCInformationDisplay.NPCInformationDisplay_C|SetDifficulty _asnpcinformation_display (Variables|AttributetoCheck|GetBasePassingValue)))

(event EventTick
  (params (DeltaSeconds :type Float%20%28single-precision%29))
  (bind _scene (Variables|Default|GetScene))
  (bind _asbp_dog (Utilities|Casting|CastToBP_Dog (Game|GetPlayerCharacter 0)))
  (Transformation|SetWorldRotation _scene (Math|Rotator|FindLookatRotation (Transformation|GetWorldLocation _scene) (Transformation|GetWorldLocation (Variables|/Game/Player+AI/Blueprints/BP_Dog.BP_Dog_C|GetFollowCamera _asbp_dog))) false false))

(event EventUseInteract
  (params (UsingActor :type Actor%20Object%20Reference))
  (bind _asbp_dog (Utilities|Casting|CastToBP_Dog UsingActor))
  (bind _passedcheck_ (CallFunction|CheckPlayerAttributes))
  (if (and _passedcheck_ (<= (Variables|Default|GetTricksDone) 1))
    (Variables|Default|SetAnim%20State "NewEnumerator5")
    (Audio|PlaySound2D "/Game/Sound/ABS/ABS_Approval_MiniGameStart.ABS_Approval_MiniGameStart" 1.0 1.0 0.0 0 0)
    (Utilities|FlowControl|Delay 1.0)
    (Default|ChooseRandomMinigame _asbp_dog)
    (else
      (Variables|Default|SetAnim%20State "NewEnumerator8")
      (Audio|PlaySound2D "/Game/Sound/ABS/ABS_Rejected.ABS_Rejected" 1.0 1.0 0.0 0 0))))

(event EventStartConversation
  (params (TalkingActor :type Master%20AI%20Object%20Reference))
  (Variables|Default|SetTalkingActor TalkingActor)
  (AI|Components|Blackboard|SetValueasBool (AI|GetBlackboard 0) (Variables|Default|GetisBeingTalkedToKey) true))

(event EventEndConversation
  (AI|Components|Blackboard|SetValueasBool (AI|GetBlackboard 0) (Variables|Default|GetisBeingTalkedToKey) false))

(fn ConstructionScript
  (|CallParentFunction))

(fn CheckPlayerAttributes
  (bind _returnvalue (AI|GetBlackboard 0))
  (bind _playerkey (Variables|Default|GetPlayerKey))
  (bind _returnvalue_2 (AI|Components|Blackboard|GetValueasObject _returnvalue _playerkey))
  (bind _asbp_dog (Utilities|Casting|CastToBP_Dog _returnvalue_2))
  (bind _playerstats (Variables|/Game/Player+AI/Blueprints/BP_Dog.BP_Dog_C|GetPlayerStats _asbp_dog))
  (switch Utilities|FlowControl|Switch|SwitchonAttributeCheckEnum (Variables|AttributeToCheck|GetAttributeCheckEnum)
    (:NewEnumerator0
      (LocalVariables|SetAttributeValue (.fancyness _playerstats)))
    (:NewEnumerator1
      (LocalVariables|SetAttributeValue (.stinkiness _playerstats)))
    (:NewEnumerator2
      (LocalVariables|SetAttributeValue (.cuteness _playerstats)))
    (:NewEnumerator3
      (LocalVariables|SetAttributeValue (.wackiness _playerstats)))
    (:NewEnumerator4
      (LocalVariables|SetAttributeValue (.coolness _playerstats))))
  (return (>= (LocalVariables|GetAttributeValue) (Variables|AttributetoCheck|GetBasePassingValue))))