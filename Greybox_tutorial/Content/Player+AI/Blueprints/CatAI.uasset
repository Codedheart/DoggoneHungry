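; Cat AI that catches the player's dog when it moves too fast nearby and in front of the cat.
; A looping timer runs a pawn capsule trace, then tests player speed and a horizontal view cone sized by DetectionDegree, with no line-of-sight check.
; Detection calls Caught on the player character, shows a CaughtMessage widget, then respawns the player and removes the message after a short delay.
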(event Custom|CaughtDog!
  (bind _as_00 (Utilities|Casting|CastTo_00 (Game|GetPlayerCharacter 0)))
  (Default|Caught _as_00)
  (bind _returnvalue (UserInterface|CreateWidget "/Game/UI/Widgets/CaughtMessage.CaughtMessage_C" (Game|GetPlayerController 0)))
  (bind _output_get (Variables|Default|SetCaughtMessage _returnvalue))
  (UserInterface|Viewport|AddtoViewport _output_get 0)
  (Utilities|FlowControl|Delay 1.5)
  (Default|Respawn _as_00)
  (Widget|RemovefromParent (Variables|Default|GetCaughtMessage)))

(event EventBeginPlay
  (Utilities|Time|SetTimerbyFunctionName 0 "DetectionTrace" 0.1 true))

(fn ConstructionScript)

(fn DetectionTrace
  (bind _returnvalue (Transformation|GetActorLocation))
  (bind _returnvalue_2 (Transformation|GetActorForwardVector))
  (bind _returnvalue_3 (Transformation|GetActorLocation))
  (bind _returnvalue_4 (Game|Player|GetPlayerPawn 0))
  (bind _returnvalue_5 (Transformation|GetActorLocation _returnvalue_4))
  (bind _returnvalue_6 (Math|Vector|GetUnitDirection(Vector) _returnvalue_3 _returnvalue_5))
  (bind _outhits (Class|KismetSystemLibrary|CapsuleTraceMultiforObjects _returnvalue _returnvalue 3e+02 1e+03 (Utilities|Array|MakeArray "ObjectTypeQuery3") false (Utilities|Array|MakeArray self) "None" true))
  (for _array_element _outhits
    (if (== (.HitActor (Collision|BreakHitResult _array_element)) _returnvalue_4)
      (if (and (> (Math|Vector|VectorLength (Transformation|GetVelocity (Game|Player|GetPlayerPawn 0))) 301.0) (< (Class|KismetMathLibrary|DegAcos (Math|Vector|DotProduct (Math|Vector|MakeVector (.x _returnvalue_6) (.y _returnvalue_6) 0.0) (Math|Vector|MakeVector (.x _returnvalue_2) (.y _returnvalue_2) 0.0))) (Variables|Default|GetDetectionDegree)))
        (CallFunction|CaughtDog!)))))