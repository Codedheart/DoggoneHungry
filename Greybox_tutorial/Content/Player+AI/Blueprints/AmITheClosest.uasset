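; AmITheClosest is an AI condition check, apparently a Behavior Tree decorator, that passes only for the AI nearest the player and within barking distance.
; It gathers all actors of the OwnerAI class and scans their distances to the player object stored in the controlled pawn's blackboard.
; It returns true when the pawn is that closest actor and its own distance is at most BarkingDistance.
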(fn PerformConditionCheckAI
  (params (OwnerController :type AI%20Controller%20Object%20Reference) (ControlledPawn :type Pawn%20Object%20Reference))
  (bind _returnvalue (AI|GetBlackboard ControlledPawn))
  (bind _playerkey (Variables|Default|GetPlayerKey))
  (bind _returnvalue_2 (AI|Components|Blackboard|GetValueasObject _returnvalue _playerkey))
  (Variables|Default|SetClosestLocation 5e+04)
  (bind _outactors (Actor|GetAllActorsOfClass "/Game/Player+AI/Blueprints/OwnerAI.OwnerAI_C"))
  (bind _output_get (Variables|Default|SetOwners _outactors))
  (bind (_array_element _array_index) (Utilities|Array|ForEachLoopwithBreak _output_get)
    (:LoopBody
      (if (< (Transformation|GetDistanceTo _array_element (.As%2000 (Utilities|Casting|CastTo_00 _returnvalue_2))) (Variables|Default|GetClosestLocation))
        (Variables|Default|SetClosestLocation (Transformation|GetDistanceTo _array_element (.As%2000 (Utilities|Casting|CastTo_00 _returnvalue_2))))
        (Variables|Default|SetClosestLocationIndex _array_index)))
    (:Completed
      (return (and (== ControlledPawn (Utilities|Array|Get(acopy) (Variables|Default|GetOwners) (Variables|Default|GetClosestLocationIndex))) (<= (Transformation|GetDistanceTo ControlledPawn (.As%2000 (Utilities|Casting|CastTo_00 _returnvalue_2))) (LocalVariables|GetBarkingDistance)))))))