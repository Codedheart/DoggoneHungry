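; Behavior tree task that turns a GuestAI pawn toward the actor it is talking to.
; It first saves the pawn's current rotation to a blackboard key so the facing can be resumed later.
; It then applies a single yaw-only RInterpTo step toward the TalkingActor and finishes successfully at once, so each execution covers only part of the turn.
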(event EventReceiveExecuteAI
  (params (OwnerController :type AI%20Controller%20Object%20Reference) (ControlledPawn :type Pawn%20Object%20Reference))
  (bind _returnvalue (Transformation|GetActorRotation ControlledPawn))
  (Class|BlackboardComponent|SetValueasRotator (AI|GetBlackboard ControlledPawn) (Variables|Default|GetInitialRotation_Key) _returnvalue) ; sets rotator for resumerotation
  (Transformation|SetActorRotation ControlledPawn (Math|Interpolation|RInterpTo _returnvalue (Math|Rotator|MakeRotator 0.0 0.0 (.Yaw (Math|Rotator|BreakRotator (Math|Rotator|FindLookatRotation (Transformation|GetActorLocation ControlledPawn) (Transformation|GetActorLocation (Variables|/Game/Player+AI/Blueprints/GuestAI.GuestAI_C|GetTalkingActor (.AsGuest%20AI (Utilities|Casting|CastToGuestAI ControlledPawn)))))))) 1.0 0.2))
  (AI|BehaviorTree|FinishExecute true))