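; Behavior tree task that claims a free bathroom for an AI guest.
; It scans actors tagged NPCPOI for the first BathroomDoor not in use and stores it in the blackboard POI key.
; A found door is marked in use, its outside arrow position becomes the location key, and the task succeeds.
; Otherwise it starts the GuestAI bathroom timer and fails.
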(event EventReceiveExecuteAI
  (params (OwnerController :type AI%20Controller%20Object%20Reference) (ControlledPawn :type Pawn%20Object%20Reference))
  (bind _returnvalue (AI|GetBlackboard ControlledPawn))
  (Variables|Default|SetTargetBathroom 0)
  (bind _outactors (Actor|GetAllActorswithTag "NPCPOI"))
  (bind _array_element (Utilities|Array|ForEachLoopwithBreak _outactors :!label _label)
    (:LoopBody
      (bind _asbathroom_door (Utilities|Casting|CastToBathroomDoor _array_element))
      (if (not (Variables|/Game/Blueprints/Interactables/BathroomDoor.BathroomDoor_C|GetinUse? _asbathroom_door)) ; Find first bathroom not in use
        (bind _output_get (Variables|Default|SetTargetBathroom _asbathroom_door))
        (AI|Components|Blackboard|SetValueasObject _returnvalue (Variables|Default|GetPOIKey) _output_get)
        (goto _label Break)))
    (:Completed
      (Utilities|IsValid (Variables|Default|GetTargetBathroom) ; Did they find a useable bathroom?
        (:Is%20Valid
          (Variables|/Game/Blueprints/Interactables/BathroomDoor.BathroomDoor_C|SetinUse? (Variables|Default|GetTargetBathroom) true)
          (AI|Components|Blackboard|SetValueasVector _returnvalue (Variables|Default|GetLocationKey) (Transformation|GetWorldLocation (Variables|/Game/Blueprints/Interactables/BathroomDoor.BathroomDoor_C|GetArrow_OUT (Variables|Default|GetTargetBathroom))))
          (AI|BehaviorTree|FinishExecute true))
        (:Is%20Not%20Valid
          (Default|StartBathroomTimer (.AsGuest%20AI (Utilities|Casting|CastToGuestAI ControlledPawn)))
          (AI|BehaviorTree|FinishExecute false))))))