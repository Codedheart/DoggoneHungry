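; TrickSequenceGuest is a guest AI Blueprint that checks whether the player dog's attribute meets a passing threshold, presumably for trick sequences.
; CheckPlayerAttributes switches on AttributeCheckEnum, reads the matching PlayerStats value from the BP_Dog stored in the blackboard, and compares it to BasePassingValue.
; The Cute branch stores Cuteness but is not wired to that comparison and return, unlike the other four attributes.
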(fn ConstructionScript
  (|CallParentFunction))

(fn CheckPlayerAttributes
  (bind _returnvalue (AI|GetBlackboard 0))
  (bind _playerkey (Variables|Default|GetPlayerKey))
  (bind _returnvalue_2 (AI|Components|Blackboard|GetValueasObject _returnvalue _playerkey))
  (bind _asbp_dog (Utilities|Casting|CastToBP_Dog _returnvalue_2))
  (bind _playerstats (Variables|/Game/Player+AI/Blueprints/BP_Dog.BP_Dog_C|GetPlayerStats _asbp_dog))
  (switch Utilities|FlowControl|Switch|SwitchonAttributeCheckEnum (Variables|AttributeToCheck|GetAttributeCheckEnum)
    (:NewEnumerator0
      (LocalVariables|SetAttributeValue (.fancyness _playerstats))
      (return (>= (LocalVariables|GetAttributeValue) (Variables|AttributetoCheck|GetBasePassingValue))))
    (:NewEnumerator1
      (LocalVariables|SetAttributeValue (.stinkiness _playerstats))
      (return (>= (LocalVariables|GetAttributeValue) (Variables|AttributetoCheck|GetBasePassingValue))))
    (:NewEnumerator2
      (LocalVariables|SetAttributeValue (.cuteness _playerstats)))
    (:NewEnumerator3
      (LocalVariables|SetAttributeValue (.wackiness _playerstats))
      (return (>= (LocalVariables|GetAttributeValue) (Variables|AttributetoCheck|GetBasePassingValue))))
    (:NewEnumerator4
      (LocalVariables|SetAttributeValue (.coolness _playerstats))
      (return (>= (LocalVariables|GetAttributeValue) (Variables|AttributetoCheck|GetBasePassingValue))))))