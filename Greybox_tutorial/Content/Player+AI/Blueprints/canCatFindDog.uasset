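; Behavior tree decorator that decides whether the AI (a cat, going by the asset name) can find the player dog.
; It reads the Player object and IsPlayerSeen flag from the blackboard.
; The check passes only when the player is seen and is either acting or moving faster than a fixed speed threshold.
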(fn PerformConditionCheckAI
  (params (OwnerController :type AI%20Controller%20Object%20Reference) (ControlledPawn :type Pawn%20Object%20Reference))
  (bind _player (Variables|Default|GetPlayer))
  (bind _returnvalue (Class|BTFunctionLibrary|GetBlackboardValueasObject _player))
  (bind _as_00 (Utilities|Casting|CastTo_00 _returnvalue))
  (return (and (or (Variables|/Game/Player+AI/Blueprints/_00._00_C|GetisActing? _as_00) (> (Math|Vector|VectorLength (Transformation|GetVelocity _as_00)) 301.0)) (Class|BTFunctionLibrary|GetBlackboardValueasBool (Variables|Default|GetisPlayerSeen?)))))