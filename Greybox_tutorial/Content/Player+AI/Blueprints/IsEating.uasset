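; IsEating is a Behavior Tree decorator that lets an AI branch run only when it can see the player and that player is eating.
; Its AI condition check reads a player-seen bool and the player object from the pawn's Blackboard through key variables.
; It casts the player to BP_Dog and passes only if both the seen flag and the dog's IsEating flag are true.
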(fn PerformConditionCheckAI
  (params (OwnerController :type AI%20Controller%20Object%20Reference) (ControlledPawn :type Pawn%20Object%20Reference))
  (bind _returnvalue (AI|GetBlackboard ControlledPawn))
  (if (and (ScalableFloat|GetValueasBool _returnvalue (LocalVariables|GetisPlayerSeen_Key)) (Variables|/Game/Player+AI/Blueprints/BP_Dog.BP_Dog_C|GetisEating? (.AsBP%20Dog (Utilities|Casting|CastToBP_Dog (AI|Components|Blackboard|GetValueasObject _returnvalue (LocalVariables|GetPlayer_Key)))))) ; if player is visible and eating
    (return true)
    (else
      (return false))))