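; Behavior tree task that walks an OwnerAI pawn through a door stored in the blackboard's POI key.
; It triggers the door's interact, moves to its InArrow, waits briefly, moves on to its OutArrow, then interacts again and succeeds.
; A non-door POI or failed move fails the task, while a pawn that is not an OwnerAI leaves it unfinished.
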(event EventReceiveExecuteAI
  (params (OwnerController :type AI%20Controller%20Object%20Reference) (ControlledPawn :type Pawn%20Object%20Reference))
  (Utilities|Casting|CastToOwnerAI ControlledPawn)
  (bind _asuseable_door_bp (Utilities|Casting|CastToUseableDoorBP (AI|BehaviorTree|GetBlackboardValueasActor (Variables|Default|GetPOIKey)))
    (:then
      (Default|UseInteract _asuseable_door_bp)
      (AI|AIMoveTo ControlledPawn (Transformation|GetWorldLocation (Variables|/Game/Blueprints/Interactables/UseableDoorBP.UseableDoorBP_C|GetInArrow _asuseable_door_bp)) 0 2.0 false
        (:OnSuccess
          (Utilities|FlowControl|Delay 2.0)
          (AI|AIMoveTo ControlledPawn (Transformation|GetWorldLocation (Variables|/Game/Blueprints/Interactables/UseableDoorBP.UseableDoorBP_C|GetOutArrow _asuseable_door_bp)) 0 2.0 false
            (:OnSuccess
              (Default|UseInteract _asuseable_door_bp)
              (AI|BehaviorTree|FinishExecute true))
            (:OnFail
              (AI|BehaviorTree|FinishExecute false))))
        (:OnFail
          (AI|BehaviorTree|FinishExecute false))))
    (:CastFailed
      (AI|BehaviorTree|FinishExecute false))))