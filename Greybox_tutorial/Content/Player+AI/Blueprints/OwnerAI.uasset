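; Owner AI Blueprint that reacts to cat calls and exposes vision settings for the owner.
; Each received cat call toggles the PunishDog blackboard key through a FlipFlop, leaving the resulting behavior to logic outside this graph.
; Separate events switch the PCaught particle on and off, and a function returns the vision radius and angle.
; POI gathering and player-distance printing are present but never run.
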(event Custom|EventRecieveCatCall
  (bind _isa (Utilities|FlowControl|FlipFlop)
    (:A
      _)
    (:B
      _))
  (AI|Components|Blackboard|SetValueasBool (AI|GetBlackboard 0) (Variables|Default|GetPunishDog) _isa))

(event Custom|ActivateParticle
  (Components|Activation|SetActive (Variables|Default|GetP_Caught) true false))

(event Custom|DeactivateParticle
  (Components|Activation|SetActive (Variables|Default|GetP_Caught) false false))

(event EventBeginPlay)

(event EventTick
  (params (DeltaSeconds :type Float%20%28single-precision%29)))

(fn ConstructionScript
  (|CallParentFunction))

(fn RetrieveVisionRangeParameters
  (return (Variables|Default|GetVisionRange) (Variables|Default|GetVisionAngle)))