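; Behavior tree task that picks the next point of interest for an OwnerAI pawn.
; It writes the entry at POIIterator in the pawn's POIArray to the POIKey blackboard key, then advances the iterator and finishes successfully.
; The iterator resets only after it has reached the array length, so one read per cycle falls past the last entry.
; A failed pawn cast never calls FinishExecute.
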(event EventReceiveExecuteAI
  (params (OwnerController :type AI%20Controller%20Object%20Reference) (ControlledPawn :type Pawn%20Object%20Reference))
  (bind _asowner_ai (Utilities|Casting|CastToOwnerAI ControlledPawn))
  (Class|BTFunctionLibrary|SetBlackboardValueasObject (Variables|Default|GetPOIKey) (Utilities|Array|Get(acopy) (Variables|/Game/Player+AI/Blueprints/OwnerAI.OwnerAI_C|GetPOIArray _asowner_ai) (Variables|Default|GetPOIIterator)))
  (if (>= (Variables|Default|GetPOIIterator) (Utilities|Array|Length (Variables|/Game/Player+AI/Blueprints/OwnerAI.OwnerAI_C|GetPOIArray _asowner_ai)))
    (Variables|Default|SetPOIIterator 0)
    (else
      (Math|Integer|IncrementInt (Variables|Default|GetPOIIterator)
        (:%20%20
          _))))
  (AI|BehaviorTree|FinishExecute true))