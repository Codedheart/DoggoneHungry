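; BadDog is a behavior tree task that plays out the owner AI catching the player.
; It switches the OwnerAI pawn's animation state and shows a CaughtMessage widget on screen for a short delay.
; It then switches the animation state again, respawns the player read from the blackboard's PlayerKey, removes the widget and finishes successfully.
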(event EventReceiveExecuteAI
  (params (OwnerController :type AI%20Controller%20Object%20Reference) (ControlledPawn :type Pawn%20Object%20Reference))
  (bind _asowner_ai (Utilities|Casting|CastToOwnerAI ControlledPawn))
  (Variables|/Game/Player+AI/Blueprints/MasterAI.MasterAI_C|SetAnim%20State _asowner_ai "NewEnumerator7")
  (bind _returnvalue (UserInterface|CreateWidget "/Game/UI/Widgets/CaughtMessage.CaughtMessage_C"))
  (bind _output_get (Variables|Default|SetCaughtMessage _returnvalue))
  (UserInterface|Viewport|AddtoViewport _output_get 0)
  (Utilities|FlowControl|Delay 1.5)
  (Variables|/Game/Player+AI/Blueprints/MasterAI.MasterAI_C|SetAnim%20State _asowner_ai "NewEnumerator0")
  (Default|Respawn (.As%2000 (Utilities|Casting|CastTo_00 (AI|Components|Blackboard|GetValueasObject (AI|GetBlackboard ControlledPawn) (Variables|Default|GetPlayerKey)))))
  (Widget|RemovefromParent (Variables|Default|GetCaughtMessage))
  (AI|BehaviorTree|FinishExecute true))