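; AI controller for the cat enemy, which runs the BTCat behavior tree and tracks the dog character as its player target.
; On BeginPlay it finds the first BP_Dog and writes that actor and its starting location to the blackboard, printing a warning if none exist.
; AI perception updates for a BP_Dog set a blackboard flag for whether the player is currently seen.
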(event OnTargetPerceptionUpdated(AIPerception)
  (params (Actor :type Actor%20Object%20Reference) (Stimulus :type AI%20Stimulus%20Structure))
  (Utilities|Casting|CastToBP_Dog Actor)
  (AI|Components|Blackboard|SetValueasBool (Variables|Default|GetBlackboard) (Variables|Default|GetisPlayerSeenKey) (.bsuccessfullysensed Stimulus)))

(event EventBeginPlay
  (AI|RunBehaviorTree "/Game/Player+AI/Blueprints/BTCat.BTCat")
  (bind _outactors (Actor|GetAllActorsOfClass "/Game/Player+AI/Blueprints/BP_Dog.BP_Dog_C"))
  (bind _output_get (Variables|Default|SetPlayerArray _outactors))
  (if (> (Utilities|Array|Length _output_get) 0)
    (AI|Components|Blackboard|SetValueasObject (AI|GetBlackboard 0) (Variables|Default|GetPlayer_Key) (Utilities|Array|Get(acopy) _output_get))
    (AI|Components|Blackboard|SetValueasVector (AI|GetBlackboard 0) (Variables|Default|GetLocation_Key) (Transformation|GetActorLocation (Utilities|Array|Get(acopy) _output_get)))
    (else
      (Development|PrintString "NO ACTORS FOUND"))))

(event EventTick
  (params (DeltaSeconds :type Float%20%28single-precision%29)))

(fn ConstructionScript
  (|CallParentFunction))