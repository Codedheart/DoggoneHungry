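; Tutorial variant of the player dog that advances the tutorial controller the first time the dog eats and first barks while overlapping that controller.
; Eating sets an animation state and, through a delay and gate, processes the food.
; Grounded barks briefly lock movement behind a resetting DoOnce.
; Turn and look input are hard-disabled, key 9 calls a random minigame, and StartTrickSequence builds a trick sequence.
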(event Custom|StartTrickSequence
  (CallFunction|ConstructTrickSequence))

(event EventBeginPlay
  (|CallParentFunction)
  (Variables|Default|SetStartTransform (Transformation|GetWorldTransform (Variables|Default|GetCameraBoom))))

(event EventTick
  (params (DeltaSeconds :type Float%20%28single-precision%29))
  (|CallParentFunction DeltaSeconds) ; This node is disabled and will not be called.\nDrag off pins to build functionality.
)

(event EventEatFood
  (params (Food :type Actor%20Object%20Reference))
  (bind _asmaster_food (Utilities|Casting|CastToMasterFood Food))
  (Variables|Default|SetisEating? true)
  (Variables|Default|SetAnimStateEnum "NewEnumerator8")
  (Utilities|FlowControl|Delay 1.0)
  (Utilities|FlowControl|Gate false
    (:Exit
      (CallFunction|AddandEatFood _asmaster_food)
      (CallFunction|CheckFood (Variables|/Game/Blueprints/Interactables/FoodBPs/MasterFood.MasterFood_C|GetFoodValue _asmaster_food))
      (Class|InteractableInterface|UseInteract(Message) Food)
      (Variables|Default|SetAnimStateEnum "NewEnumerator0")
      (Variables|Default|SetisEating? false)
      (if (not (Variables|Default|GetbHasEatenFood))
        (Variables|Default|SetbHasEatenFood true)
        (Default|NextTaskforTutorial (Variables|Default|GetTutorialController_0))))))

(event Input|ActionEvents|InputActionBark
  (params (Key :type Key%20Structure))
  (bind _charactermovement (Variables|Character|GetCharacterMovement))
  (:Pressed
    (if (not (AI|Components|NavMovement|IsFalling (Variables|Character|GetCharacterMovement)))
      (Utilities|FlowControl|DoOnce false :!label _label
        (:Completed
          (Variables|Default|SetisActing? true)
          (Pawn|Components|CharacterMovement|DisableMovement _charactermovement)
          (if (and (Collision|IsOverlappingActor (Variables|Default|GetTutorialController_0) :!class /Script/Engine.Actor) (not (Variables|Default|GetbHasBarked)))
            (Default|NextTaskforTutorial (Variables|Default|GetTutorialController_0))
            (Variables|Default|SetbHasBarked true))
          (Utilities|FlowControl|Delay 1.2)
          (Variables|Default|SetisActing? false)
          (Pawn|Components|CharacterMovement|SetMovementMode _charactermovement "MOVE_Walking" 0)
          (goto _label Reset))))))

(event Input|AxisEvents|InputAxisTurn
  (params (AxisValue :type Float%20%28single-precision%29))
  (if (not true)
    (Pawn|Input|AddControllerYawInput AxisValue)))

(event Input|AxisEvents|InputAxisLookUp
  (params (AxisValue :type Float%20%28single-precision%29))
  (if (not true)
    (Pawn|Input|AddControllerPitchInput AxisValue)))

(event Input|KeyboardEvents|9
  (params (Key :type Key%20Structure))
  (:Pressed
    (CallFunction|ChooseRandomMinigame -1)))

(fn ConstructionScript
  (|CallParentFunction))