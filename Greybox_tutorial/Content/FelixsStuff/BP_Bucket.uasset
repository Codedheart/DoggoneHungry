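; BP_Bucket is a bucket that tips over and leads to a watermelon appearing, triggered by interaction or by a BP_Dog overlapping its capsule.
; Both triggers share one delayed sequence that rotates the bucket and then enables physics simulation on it.
; It then spawns a temporary water plane, destroys it after a few seconds and spawns the watermelon.
; Both spawns use hard-coded transforms rather than positions derived from the bucket.
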(event OnComponentBeginOverlap(Capsule)
  (params (OverlappedComponent :type Primitive%20Component%20Object%20Reference) (OtherActor :type Actor%20Object%20Reference) (OtherComp :type Primitive%20Component%20Object%20Reference) (OtherBodyIndex :type Integer) (bFromSweep :type Boolean) (SweepResult :type Hit%20Result%20Structure%20%28by%20ref%29))
  (Utilities|Casting|CastToBP_Dog OtherActor)
  (Transformation|SetRelativeLocationAndRotation (Variables|Default|GetBucket) "0, 0, 0" "50.000000, 0, 0" false false)
  (Utilities|FlowControl|Delay 0.2)
  (Physics|SetSimulatePhysics (Variables|Default|GetBucket) true)
  (Utilities|FlowControl|Delay 1.0)
  (bind _returnvalue (Game|SpawnActorfromClass "/Game/FelixsStuff/Waterplane.Waterplane_C" (Math|Transform|MakeTransform "165.000000,2945.000000,35.000000" "0, 0, 0" "0.800000,0.800000,0.800000") "Undefined" 0 0))
  (Utilities|FlowControl|Delay 3.0)
  (Actor|DestroyActor _returnvalue)
  (Game|SpawnActorfromClass "/Game/FelixsStuff/WaterMelon.WaterMelon_C" (Math|Transform|MakeTransform "170.000000,2950.000000,43.638603" "0, 0, 0" "1,1,1") "Undefined" 0 0))

(event EventUseInteract
  (params (UsingActor :type Actor%20Object%20Reference))
  (Transformation|SetRelativeLocationAndRotation (Variables|Default|GetBucket) "0, 0, 0" "50.000000, 0, 0" false false)
  (Utilities|FlowControl|Delay 0.2)
  (Physics|SetSimulatePhysics (Variables|Default|GetBucket) true)
  (Utilities|FlowControl|Delay 1.0)
  (bind _returnvalue (Game|SpawnActorfromClass "/Game/FelixsStuff/Waterplane.Waterplane_C" (Math|Transform|MakeTransform "165.000000,2945.000000,35.000000" "0, 0, 0" "0.800000,0.800000,0.800000") "Undefined" 0 0))
  (Utilities|FlowControl|Delay 3.0)
  (Actor|DestroyActor _returnvalue)
  (Game|SpawnActorfromClass "/Game/FelixsStuff/WaterMelon.WaterMelon_C" (Math|Transform|MakeTransform "170.000000,2950.000000,43.638603" "0, 0, 0" "1,1,1") "Undefined" 0 0))

(fn ConstructionScript)